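; Crafting component that turns grass dropped into the bowl into an effect for the player.
; It tracks the clicked grass, drops it on release and fills the bowl if the cursor trace hits it.
; A full bowl is checked against CraftingRecepies_DT rows as an order-independent two-ingredient match.
; A match shows the effect, stores it in the controller's StateBeforeSitting and removes the used inventory items.
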(event EventBeginPlay
  (CallFunction|SetRefs))

(fn SetRefs
  (bind _asmain_pc (Utilities|Casting|CastToMain_PC (Game|GetPlayerController 0)))
  (bind _output_get (Variables|Refs|SetPC_Ref _asmain_pc))
  (Variables|Refs|SetBowl_Ref (Variables|/Game/Blueprints/Generic/Main_PC.Main_PC_C|GetBowl_Ref _output_get))
  (Variables|Refs|SetInventoryComponent_Ref (Variables|/Game/Blueprints/Character/Main_Character.Main_Character_C|GetInventory_Component (.AsMain%20Character (Utilities|Casting|CastToMain_Character (Game|GetPlayerCharacter 0))))))

(fn FillSelected
  (params (lastClicked :type Clicked%20Grass%20S%20Structure))
  (Variables|Default|SetLastClicked lastClicked))

(fn EmptySelected
  (Variables|Default|SetLastClicked ""))

(fn Produce
  (bind _grassforcraft (Variables|Default|GetGrassForCraft))
  (bind (_craftable _effect) (CallFunction|CheckifCraftableandEffect _grassforcraft))
  (if _craftable
    ;[1 1 1] For now
    (Default|ShowGainedEffect (Variables|Refs|GetBowl_Ref) _effect)
    (Variables|/Game/Blueprints/Generic/Main_PC.Main_PC_C|SetstateBeforeSitting (Variables|Refs|GetPC_Ref) _effect)
    ;[1 1 1] TODO: Use dispatcher?
    (for _array_element (Variables|/Game/Blueprints/World/Craft/Bowl_BP.Bowl_BP_C|GetGrassInBowl (Variables|Refs|GetBowl_Ref))
      (Default|RemoveElement (Variables|Refs|GetInventoryComponent_Ref) (.InventoryIndex (Utilities|Struct|BreakClickedGrass_S _array_element))))
    (else
      (Development|PrintString "No recipe for this" true true "(R=0.000000,G=0.658824,B=1.000000,A=1.000000)"))))

(fn DecideWhattoDo
  (bind _bowl_ref (Variables|Refs|GetBowl_Ref))
  ;[1 1 1] TODO: RENAME
  (if (CallFunction|IsHoldingSomething)
    (Default|Fall (.object (Variables|Default|GetLastClicked)))
    (if (CallFunction|IsAboveBowl)
      (Default|FillBowl (Variables|Refs|GetBowl_Ref))
      (CallFunction|EmptySelected)
      (if (Default|CheckifBowlIsFull _bowl_ref)
        (CallFunction|UpdateGrassforCraft (Variables|/Game/Blueprints/World/Craft/Bowl_BP.Bowl_BP_C|GetGrassInBowl _bowl_ref))
        (CallFunction|Produce))
      (else
        (CallFunction|EmptySelected)))))

(fn UpdateGrassforCraft
  (params (GrassForCraft :type Array%20of%20Clicked%20Grass%20S%20Structures))
  (Variables|Default|SetGrassForCraft GrassForCraft))

(fn CheckElements
  (params (RecipeInCheck :type Array%20of%20Strings) (GrassInBowl :type Array%20of%20Clicked%20Grass%20S%20Structures))
  (if (or (and (CallFunction|CheckElement RecipeInCheck GrassInBowl) (CallFunction|CheckElement RecipeInCheck GrassInBowl 1 1)) (and (CallFunction|CheckElement RecipeInCheck GrassInBowl 1) (CallFunction|CheckElement RecipeInCheck GrassInBowl 0 1)))
    (return true)
    (else
      (return false))))

(fn CheckElement
  (params (Recipe :type Array%20of%20Strings) (Grass :type Array%20of%20Clicked%20Grass%20S%20Structures) (RecipeElemIndex :type Integer) (GrassElemIndex :type Integer))
  (return (Utilities|Enum|Equal(Enum) (Utilities|Array|Get(acopy) Recipe RecipeElemIndex) (Utilities|String|EnumtoString (.Name (Utilities|Struct|BreakClickedGrass_S (Utilities|Array|Get(acopy) Grass GrassElemIndex)))))))

(fn CheckifSomethingIsSelected
  (if (== (.object (Variables|Default|GetLastClicked)) 0)
    (return false)
    (else
      (return true))))

(fn CheckifCanbeSelected
  (params (GrassInCheck :type Craft%20Grass%20Base%20BP%20Object%20Reference))
  (LocalVariables|SetGrassInCheckLocal GrassInCheck)
  (if (CallFunction|CheckifSomethingIsSelected)
    (if (== (.object (Variables|Default|GetLastClicked)) (LocalVariables|GetGrassInCheckLocal))
      (return true)
      (else
        (return false)))
    (else
      (return true))))

(fn CheckifCraftableandEffect
  (params (Grass :type Array%20of%20Clicked%20Grass%20S%20Structures))
  (bind _outrownames (DataTable|GetDataTableRowNames "/Game/Data/DataTables/CraftingRecepies_DT.CraftingRecepies_DT"))
  (for _array_element _outrownames
    (if (.Matched (CallFunction|CheckRecipe _array_element))
      (return true (.Effect (CallFunction|CheckRecipe _array_element))))))

(fn CheckRecipe
  (params (RowName :type Name))
  (bind _returnvalue (Utilities|GetDataTableRow "/Game/Data/DataTables/CraftingRecepies_DT.CraftingRecepies_DT" RowName)
    (:then
      (return (.Effect (Utilities|Struct|BreakCraftingRecipes_S _returnvalue)) (CallFunction|CheckElements (.Ingredients (Utilities|Struct|BreakCraftingRecipes_S _returnvalue)) (Variables|Default|GetGrassForCraft))))))

(fn IsAboveBowl
  (Utilities|Casting|CastToBowl_BP (.HitActor (Collision|BreakHitResult (.HitResult (Game|Player|GetHitResultUnderCursorbyChannel (Variables|Refs|GetPC_Ref) "TraceTypeQuery1" true))))
    (:then
      (return true))
    (:CastFailed
      (return false))))

(fn IsHoldingSomething
  (return (not (== (.object (Variables|Default|GetLastClicked)) 0))))