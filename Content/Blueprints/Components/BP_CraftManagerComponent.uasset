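; Crafting manager component that tracks the held grass and lets the player combine grass in a bowl to produce an effect.
; PerformCraftAction drops the held grass, filling the bowl if above it, and triggers production once the bowl is full.
; Production scans DT_CraftingRecepies for an order-independent two-ingredient match.
; A match stores the effect in the player controller's StateBeforeSitting and clears the bowl, while a miss prints a message.
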(event EventBeginPlay
  (CallFunction|SetRefs))

(fn SetRefs
  (Utilities|FlowControl|Sequence
    (:then_0
      (bind _asbp_main_pc (Utilities|Casting|CastToBP_MainPC (Game|GetPlayerController 0)))
      (bind _output_get (Variables|Refs|SetPC_Ref _asbp_main_pc))
      (Variables|Refs|SetBowl_Ref (Variables|/Game/Blueprints/Generic/BP_MainPC.BP_MainPC_C|GetBowl_Ref _output_get)))
    (:then_1
      (bind _asbp_main_character (Utilities|Casting|CastToBP_MainCharacter (Game|GetPlayerCharacter 0)))
      (Variables|Refs|SetInventoryComponent_Ref (Variables|/Game/Blueprints/Character/BP_MainCharacter.BP_MainCharacter_C|GetInventory _asbp_main_character)))))

(fn FillSelected
  (params (lastClicked :type S%20Clicked%20Grass%20Structure))
  (bind _output_get (Variables|Default|SetLastClicked lastClicked)))

(fn EmptySelected
  ;[1 1 1] For now
  (Collision|SetCollisionEnabled (Variables|/Game/Blueprints/World/Takables/Grass/BP_G_CraftGrass_Base.BP_G_CraftGrass_Base_C|GetGrassMesh (.Actor (Utilities|Struct|BreakSClickedGrass (Variables|Default|GetLastClicked)))) "QueryAndPhysics")
  (Variables|Default|SetLastClicked ""))

(fn SetIsAboveBowl
  (params (IsAbove :type Boolean))
  (Variables|Default|SetisAboveBowl IsAbove))

(fn Produce
  (bind _grassforcraft (Variables|Default|GetGrassForCraft))
  (bind (_craftable _effect) (CallFunction|CheckEffectifCraftable _grassforcraft))
  (if _craftable
    (Variables|/Game/Blueprints/Generic/BP_MainPC.BP_MainPC_C|SetstateBeforeSitting (Variables|Refs|GetPC_Ref) _effect)
    (Default|ClearBowlwithEffects (Variables|Refs|GetBowl_Ref))
    (else
      (Development|PrintString "No recipe for this" true true "(R=0.000000,G=0.658824,B=1.000000,A=1.000000)")
      (Default|ShowNumberOfGrass (Variables|/Game/Blueprints/Generic/BP_MainPC.BP_MainPC_C|GetBowl_Ref (Variables|Refs|GetPC_Ref))))))

(fn PerformCraftAction
  (bind _bowl_ref (Variables|Refs|GetBowl_Ref))
  (Development|PrintString "Perform Craft Action")
  (if (CallFunction|IsHoldingSomething)
    (Default|Fall (.actor (Variables|Default|GetLastClicked)))
    (if (Variables|Default|GetisAboveBowl)
      (Default|FillBowl (Variables|Refs|GetBowl_Ref))
      (CallFunction|EmptySelected)
      ;[1 1 1] TODO: refactor
      (if (Default|CheckifBowlIsFull _bowl_ref)
        (CallFunction|UpdateGrassforCraft (Variables|/Game/Blueprints/World/Craft/BP_Bowl.BP_Bowl_C|GetGrassInBowl _bowl_ref))
        (Default|ShowWater _bowl_ref)
        (CallFunction|Produce))
      (else
        (CallFunction|EmptySelected)))))

(fn UpdateGrassforCraft
  (params (GrassForCraft :type Array%20of%20S%20Clicked%20Grass%20Structures))
  (Variables|Default|SetGrassForCraft GrassForCraft))

(fn CheckElements
  (params (ERecipeInCheck :type Array%20of%20EGrassTypes%20Enums :default "NewEnumerator6") (GrassInBowl :type Array%20of%20S%20Clicked%20Grass%20Structures))
  (if (or (and (CallFunction|CheckElement ERecipeInCheck GrassInBowl) (CallFunction|CheckElement ERecipeInCheck GrassInBowl 1 1)) (and (CallFunction|CheckElement ERecipeInCheck GrassInBowl 1) (CallFunction|CheckElement ERecipeInCheck GrassInBowl 0 1)))
    (return true)
    (else
      (return false))))

(fn CheckElement
  (params (ERecipe :type Array%20of%20EGrassTypes%20Enums :default "NewEnumerator6") (Grass :type Array%20of%20S%20Clicked%20Grass%20Structures) (RecipeElemIndex :type Integer) (GrassElemIndex :type Integer))
  (return (Utilities|Enum|Equal(Enum) (Utilities|Array|Get(acopy) ERecipe RecipeElemIndex) (.Name (Utilities|Struct|BreakSClickedGrass (Utilities|Array|Get(acopy) Grass GrassElemIndex))))))

(fn CheckifCanbeSelected
  (params (GrassInCheck :type BP%20G%20Craft%20Grass%20Base%20Object%20Reference))
  (if (CallFunction|IsHoldingSomething)
    (if (== (.actor (Variables|Default|GetLastClicked)) GrassInCheck)
      (return true)
      (else
        (return false)))
    (else
      (return true))))

(fn CheckEffectifCraftable
  (params (Grass :type Array%20of%20S%20Clicked%20Grass%20Structures))
  (bind _outrownames (DataTable|GetDataTableRowNames "/Game/Data/DataTables/Book/DT_CraftingRecepies.DT_CraftingRecepies"))
  (for _array_element _outrownames
    (if (.Matched (CallFunction|CheckRecipe _array_element))
      (return true (.Effect (CallFunction|CheckRecipe _array_element)))))
  (return false "NewEnumerator0"))

(fn CheckRecipe
  (params (RowName :type Name))
  (bind _returnvalue (Utilities|GetDataTableRow "/Game/Data/DataTables/Book/DT_CraftingRecepies.DT_CraftingRecepies" RowName)
    (:then
      (return (.Effect (Utilities|Struct|BreakSCraftingRecipes _returnvalue)) (CallFunction|CheckElements (.Ingredients (Utilities|Struct|BreakSCraftingRecipes _returnvalue)) (Variables|Default|GetGrassForCraft))))))

(fn IsHoldingSomething
  (return (Utilities|IsValid (.actor (Variables|Default|GetLastClicked)))))