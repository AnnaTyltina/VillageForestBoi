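; Inventory component that stores collected grass types in a slot array, sized to a maximum when play begins.
; Adding looks up a row in the grass data table and fills the first slot lacking a valid craft actor class.
; Removal deletes the array element, shrinking the slot count instead of clearing it.
; It also caches player controller and character references, plus the craft manager via a controller event.
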(event Custom|SetCraftManagerRef
  ;[1 1 1] Not sure if needed
  (Variables|Refs|SetCraftManager_Ref (Variables|/Game/Blueprints/Generic/Main_PC.Main_PC_C|GetCraftManagerComponent (Variables|Refs|GetPC_Ref))))

(event EventBeginPlay
  (Development|PrintString "Inventory is here")
  (CallFunction|SetRefs)
  (CallFunction|LimitInventory)
  ;[1 1 1] Not sure if needed
  (EventDispatchers|BindEventtoOnCraftManagerAddedD (Variables|Refs|GetPC_Ref) (delegate Custom|SetCraftManagerRef)))

(fn SetRefs
  (bind _asmain_pc (Utilities|Casting|CastToMain_PC (Game|GetPlayerController 0)))
  (Variables|Refs|SetPC_Ref _asmain_pc)
  (bind _asmain_character (Utilities|Casting|CastToMain_Character (Game|GetPlayerCharacter 0)))
  (Variables|Refs|SetChar_Ref _asmain_character))

(fn LimitInventory
  (Utilities|Array|Resize (Variables|Default|GetGrassSlots) (Variables|Default|GetMaxAmountOfGrass)))

(fn AddtoInventory
  (params (Row :type Name))
  (bind _returnvalue (Utilities|GetDataTableRow "/Game/Data/DataTables/AllGrassTypes_DT.AllGrassTypes_DT" Row)
    (:then
      ;[1 1 1] Set locals
      (LocalVariables|SetGrassIndex_Local (.index _returnvalue))
      (LocalVariables|SetGrassName_Local (.name _returnvalue))
      (LocalVariables|SetGrassActor_Local (.actorforcraft _returnvalue))
      (bind (_success _index) (CallFunction|SearchforEmptySlot))
      (if _success
        ;[1 1 1] Set local
        (LocalVariables|SetEmptySlotIndex_Local _index)
        (Utilities|Array|SetArrayElem (Variables|Default|GetGrassSlots) (LocalVariables|GetEmptySlotIndex_Local) (Utilities|Struct|MakeGrassAttributes_S (LocalVariables|GetGrassIndex_Local) (LocalVariables|GetGrassName_Local) 0 (LocalVariables|GetGrassActor_Local)))
        (Development|PrintString (Utilities|String|Append (Utilities|String|EnumtoString (LocalVariables|GetGrassName_Local)) " added to " (Utilities|String|ToString(Integer) (LocalVariables|GetEmptySlotIndex_Local)) " slot"))
        (return true)
        (else
          (Development|PrintString "INVENTORY IS FULL" true true "(R=0.625000,G=0.000000,B=0.000000,A=1.000000)")
          (return false))))
    (:RowNotFound
      (Development|PrintString "NO SUCH GRASS" true true "(R=0.625000,G=0.000000,B=0.000000,A=1.000000)")
      (return false))))

(fn RemovefromInventory
  (params (SlotIndex :type Integer))
  (Utilities|Array|RemoveIndex (Variables|Default|GetGrassSlots) SlotIndex))

(fn SearchforEmptySlot
  ;[1 1 1] TODO: Refactor?
  (bind (_array_element _array_index) (Utilities|Array|ForEachLoopwithBreak (Variables|Default|GetGrassSlots) :!label _label)
    (:LoopBody
      (if (not (Utilities|IsValidClass (.actorforcraft _array_element)))
        (LocalVariables|SetFoundEmptySlot_Local true)
        (LocalVariables|SetEmptySlotIndex_Local _array_index)
        (goto _label Break)))
    (:Completed
      (return (LocalVariables|GetFoundEmptySlot_Local) (LocalVariables|GetEmptySlotIndex_Local)))))

(fn IsSlotEmpty
  (params (Index :type Integer))
  (return (not (Utilities|IsValidClass (.actorforcraft (Utilities|Array|Get(acopy) (Variables|Default|GetGrassSlots) Index))))))

(fn GetGrassAttributesbyIndex
  (params (Index :type Integer))
  (bind _grassslots (Variables|Default|GetGrassSlots))
  (bind _output (Utilities|Array|Get(acopy) _grassslots Index))
  (return (.index _output) (.name _output) (.actorforcraft _output)))