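; Inventory component that stores the player's grass and object items in two separate, size-limited slot arrays.
; BeginPlay caches player references, then clears and resizes both arrays to their maximums.
; AddToInventory finds the item's data table row by index and copies it into the first empty slot, identified by an invalid mesh.
; RemoveElement blanks grass slots only and refreshes the craft menu; debug prints remain throughout.
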(event EventBeginPlay
  (CallFunction|SetRefs)
  (CallFunction|ClearInventory)
  (CallFunction|LimitInventory)
  ;[1 0 0.9595] Debug
  (Utilities|FlowControl|Delay 1e+01)
  (for _array_element (Variables|Default|GetGrassSlots)
    (Development|PrintString (Utilities|String|ToString(Integer) (.Index (Utilities|Struct|BreakSGrassAttributes _array_element))))))

(fn SetRefs
  (Utilities|FlowControl|Sequence
    (:then_0
      (bind _asbp_main_pc (Utilities|Casting|CastToBP_MainPC (Game|GetPlayerController 0)))
      (Variables|Refs|SetPC_Ref _asbp_main_pc))
    (:then_1
      (bind _asbp_main_character (Utilities|Casting|CastToBP_MainCharacter (Game|GetPlayerCharacter 0)))
      (Variables|Refs|SetChar_Ref _asbp_main_character))))

(fn LimitInventory
  (Utilities|Array|Resize (Variables|Default|GetGrassSlots) (Variables|Default|GetMaxAmountOfGrass))
  (Utilities|Array|Resize (Variables|Default|GetObjectsSlots) (Variables|Default|GetMaxAmountOfObjects)))

(fn ClearInventory
  (Utilities|Array|Clear (Variables|Default|GetGrassSlots))
  (Utilities|Array|Clear (Variables|Default|GetObjectsSlots)))

(fn AddtoInventory
  (params (GrassIndex :type Integer) (ObjectIndex :type Integer) (Type :type EAllTakableTypes%20Enum :default "NewEnumerator0"))
  (switch Utilities|FlowControl|Switch|SwitchonEAllTakableTypes Type
    (:NewEnumerator0
      ;[1 1 1] Add Grass to inventory
      (bind _outrownames (DataTable|GetDataTableRowNames "/Game/Data/DataTables/DT_AllGrass.DT_AllGrass"))
      (for _array_element _outrownames
        (bind _returnvalue (Utilities|GetDataTableRow "/Game/Data/DataTables/DT_AllGrass.DT_AllGrass" _array_element)
          (:then
            (LocalVariables|SetGrassRowInCheck_Local _returnvalue)
            (if (== GrassIndex (.Index (Utilities|Struct|BreakSGrassAttributes _returnvalue)))
              (bind (_success _index) (CallFunction|SearchforEmptySlot Type))
              (if _success
                (LocalVariables|SetEmptySlotIndex_Local _index)
                (Utilities|Array|SetArrayElem (Variables|Default|GetGrassSlots) (LocalVariables|GetEmptySlotIndex_Local) (Utilities|Struct|MakeSGrassAttributes (.Index (Utilities|Struct|BreakSGrassAttributes (LocalVariables|GetGrassRowInCheck_Local))) (.Name (Utilities|Struct|BreakSGrassAttributes (LocalVariables|GetGrassRowInCheck_Local))) 0 (.MeshInInventory (Utilities|Struct|BreakSGrassAttributes (LocalVariables|GetGrassRowInCheck_Local)))))
                ;;[1 0 0.6584] Debug
                (Development|PrintString (Utilities|String|Append (Utilities|String|EnumtoString (.name (LocalVariables|GetGrassRowInCheck_Local))) " added to " (Utilities|String|ToString(Integer) (LocalVariables|GetEmptySlotIndex_Local)) " slot"))
                (return true)
                (else
                  (Development|PrintString "GRASS INVENTORY IS FULL" true true "(R=0.625000,G=0.000000,B=0.000000,A=1.000000)")
                  (return false))))))))
    (:NewEnumerator1
      ;[1 1 1] Add Object to inventory
      (bind _outrownames_2 (DataTable|GetDataTableRowNames "/Game/Data/DataTables/DT_AllObjects.DT_AllObjects"))
      (for _array_element_2 _outrownames_2
        (bind _returnvalue_2 (Utilities|GetDataTableRow "/Game/Data/DataTables/DT_AllObjects.DT_AllObjects" _array_element_2)
          (:then
            (LocalVariables|SetObjectRowInCheck_Local _returnvalue_2)
            (if (== ObjectIndex (.Index (Utilities|Struct|BreakSObjectAttributes _returnvalue_2)))
              (bind (_success_2 _index_2) (CallFunction|SearchforEmptySlot Type))
              (if _success_2
                (LocalVariables|SetEmptySlotIndex_Local _index_2)
                (Utilities|Array|SetArrayElem (Variables|Default|GetObjectsSlots) (LocalVariables|GetEmptySlotIndex_Local) (Utilities|Struct|MakeSObjectAttributes (.Index (Utilities|Struct|BreakSObjectAttributes (LocalVariables|GetObjectRowInCheck_Local))) (.Name (Utilities|Struct|BreakSObjectAttributes (LocalVariables|GetObjectRowInCheck_Local))) 0 (.CraftMesh (Utilities|Struct|BreakSObjectAttributes (LocalVariables|GetObjectRowInCheck_Local)))))
                ;;[1 0 0.6584] Debug
                (Development|PrintString (Utilities|String|Append (Utilities|String|EnumtoString (.name (LocalVariables|GetObjectRowInCheck_Local))) " added to " (Utilities|String|ToString(Integer) (LocalVariables|GetEmptySlotIndex_Local)) " object slot"))
                (return true)
                (else
                  (Development|PrintString "OBJ INVENTORY IS FULL" true true "(R=0.625000,G=0.000000,B=0.000000,A=1.000000)")
                  (return false))))))))))

(fn RemoveElement
  (params (SlotIndex :type Integer))
  (Utilities|Array|SetArrayElem :TargetArray (Variables|Default|GetGrassSlots) :Index SlotIndex)
  (Default|UpdateInventorySlots (Variables|Refs|GetCraftMenu_Ref)))

(fn SearchforEmptySlot
  (params (Type :type EAllTakableTypes%20Enum :default "NewEnumerator0"))
  ;[1 1 1] TODO: Refactor
  (switch Utilities|FlowControl|Switch|SwitchonEAllTakableTypes Type
    (:NewEnumerator0
      (bind (_array_element _array_index) (Utilities|Array|ForEachLoopwithBreak (Variables|Default|GetGrassSlots) :!label _label)
        (:LoopBody
          (if (not (Utilities|IsValid (.meshininventory _array_element)))
            (LocalVariables|SetFoundEmptySlot_Local true)
            (LocalVariables|SetEmptySlotIndex_Local _array_index)
            (goto _label Break)))
        (:Completed
          (return (LocalVariables|GetFoundEmptySlot_Local) (LocalVariables|GetEmptySlotIndex_Local)))))
    (:NewEnumerator1
      (bind (_array_element_2 _array_index_2) (Utilities|Array|ForEachLoopwithBreak (Variables|Default|GetObjectsSlots) :!label _label_2)
        (:LoopBody
          (if (not (Utilities|IsValid (.craftmesh _array_element_2)))
            (LocalVariables|SetFoundEmptySlot_Local true)
            (LocalVariables|SetEmptySlotIndex_Local _array_index_2)
            (goto _label_2 Break)))
        (:Completed
          (return (LocalVariables|GetFoundEmptySlot_Local) (LocalVariables|GetEmptySlotIndex_Local)))))))

(fn IsSlotEmpty
  (params (Index :type Integer) (Type :type EAllTakableTypes%20Enum :default "NewEnumerator0"))
  (switch Utilities|FlowControl|Switch|SwitchonEAllTakableTypes Type
    (:NewEnumerator0
      (return (not (Utilities|IsValid (.meshininventory (Utilities|Array|Get(acopy) (Variables|Default|GetGrassSlots) Index))))))
    (:NewEnumerator1
      (return (not (Utilities|IsValid (.craftmesh (Utilities|Array|Get(acopy) (Variables|Default|GetObjectsSlots) Index))))))))