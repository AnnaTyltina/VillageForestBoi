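; Achievements component that unlocks achievements by showing them in the achievements menu inside the pause menu.
; Shortly after BeginPlay it caches that menu through the main player controller's HUD.
; Each unlock increments a counter, which triggers a completion achievement once it reaches a threshold.
; A milk achievement unlocks only when both granny-help flags are set, otherwise it prints their values for debugging.
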(event Custom|unlockAchievement
  (params (Achievement :type EAchievements%20Enum :default "NewEnumerator0"))
  (Default|ShowAchievement (Variables|Default|GetAchievementsMenu_Ref) Achievement)
  ;[1 1 1] AllOfThem
  (bind _result (Math|Integer|IncrementInt (Variables|Default|GetachievementsCounter))
    (:%20%20
      (if (>= _result 5)
        (Default|ShowAchievement (Variables|Default|GetAchievementsMenu_Ref) "NewEnumerator5")))))

(event Custom|tryToUnlockMilkAchievement
  (if (and (Math|Boolean|Equal(Boolean) (Variables|Default|GethelpedGrandma) true) (Math|Boolean|Equal(Boolean) (Variables|Default|GethelpedReadingGranny) true))
    (CallFunction|UnlockAchievement "NewEnumerator3")
    (else
      ;[1 0 0.7199] Debug
      (Development|PrintString (Utilities|String|Append (Utilities|String|ToString(Boolean) (Variables|Default|GethelpedGrandma)) "" ", granny: " (Utilities|String|ToString(Boolean) (Variables|Default|GethelpedReadingGranny)))))))

(event EventBeginPlay
  (Utilities|FlowControl|Delay 0.2)
  (CallFunction|SetRef))

(fn SetRef
  (bind _asbp_main_pc (Utilities|Casting|CastToBP_MainPC (Game|GetPlayerController 0)))
  (Variables|Default|SetAchievementsMenu_Ref (Variables|/Game/Blueprints/Widgets/Menus/MainMenu/WBP_PauseMenu.WBP_PauseMenu_C|GetWBP_AchievementsMenu (Variables|/Game/Blueprints/Widgets/WBP_HUD.WBP_HUD_C|GetWBP_PauseMenu (Variables|/Game/Blueprints/Generic/BP_MainPC.BP_MainPC_C|GetHUD_Ref _asbp_main_pc)))))