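; BP_NPC_Base is a base NPC Blueprint that opens dialogue when the main character walks into its talk trigger.
; On BeginPlay, SetRefs caches the player controller and main character as PCRef and CharRef.
; When TalkTrigger overlaps BP_MainCharacter, it calls ShowDialogue on the cached controller, passing itself as the speaker.
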(event OnComponentBeginOverlap(TalkTrigger)
  (params (OverlappedComponent :type Primitive%20Component%20Object%20Reference) (OtherActor :type Actor%20Object%20Reference) (OtherComp :type Primitive%20Component%20Object%20Reference) (OtherBodyIndex :type Integer) (bFromSweep :type Boolean) (SweepResult :type Hit%20Result%20Structure%20%28by%20ref%29))
  (Utilities|Casting|CastToBP_MainCharacter OtherActor)
  (Default|ShowDialogue (Variables|Refs|GetPC_Ref) self))

(event EventBeginPlay
  (CallFunction|SetRefs))

(fn ConstructionScript)

(fn SetRefs
  (bind _asbp_main_pc (Utilities|Casting|CastToBP_MainPC (Game|GetPlayerController 0)))
  (Variables|Refs|SetPC_Ref _asbp_main_pc)
  (bind _asbp_main_character (Utilities|Casting|CastToBP_MainCharacter (Game|GetPlayerCharacter 0)))
  (Variables|Refs|SetChar_Ref _asbp_main_character))