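; GrassBase_BP is a base grass actor that can be selected for crafting and held by the character, with its mesh chosen from Attributes.VisualForm at construction.
; Clicking passes it to the player controller's CraftManagerComponent and, if selection is allowed, attaches it to the character's HoldingSocket.
; Fall uses a timeline to sweep it down to world Z zero, then detaches it.
; Controller and character references are cached on BeginPlay, with test-controller scaffolding still present.
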(event Custom|Respond
  (Development|PrintString "Was taken")
  (if (Default|CheckifCanbeSelected (Variables|/Game/Blueprints/Generic/Main_PC.Main_PC_C|GetCraftManagerComponent (Variables|Refs|GetMainPC_Ref)) self)
    (Default|FillSelected (Variables|/Game/Blueprints/Generic/Main_PC.Main_PC_C|GetCraftManagerComponent (Variables|Refs|GetMainPC_Ref)) self)
    ;[1 1 1] TODO: Move
    (CallFunction|TakeinHand)))

(event Custom|StopResponding
  (Development|PrintString "Was dropped")
  (Transformation|DetachFromComponent (Variables|Default|GetScene) "KeepWorld" "KeepWorld" "KeepWorld" true))

(event Custom|Fall
  (bind _returnvalue (Transformation|GetActorLocation))
  ;[1 1 1] TODO: mind collision or (worse) get CraftBlanket height
  (bind _alpha (Timeline|FallTimeline PlayFromStart)
    (:Update
      (Transformation|SetActorLocation (Math|Vector|MakeVector (.x _returnvalue) (.y _returnvalue) (Math|Float|Lerp (.z _returnvalue) 0.0 _alpha)) true false))
    (:Finished
      (CallFunction|StopResponding))))

(event MouseInput|EventActorOnClicked
  (params (ButtonPressed :type Key%20Structure :default "None"))
  (Development|PrintString "Grass clicked")
  (CallFunction|Respond)
  (Default|FillSelected (Variables|/Game/Blueprints/Generic/Main_PC.Main_PC_C|GetCraftManagerComponent (Variables|Refs|GetMainPC_Ref)) self))

(event EventBeginPlay
  (CallFunction|SetRefs))

(fn ConstructionScript
  (Components|StaticMesh|SetStaticMesh (Variables|Default|GetStaticMesh) (Utilities|Select :Index (.visualform (Variables|Default|GetAttributes)) :NewEnumerator0 "/Game/Assets/Meshes/1M_Cube.1M_Cube" :NewEnumerator1 "/Game/Testing/TestGrass_Mesh.TestGrass_Mesh" :NewEnumerator2 "/Engine/BasicShapes/Cone.Cone")))

(fn SetRefs
  ;[1 1 1] DON'T FORGET TO CHANGE PC
  (bind _astest_craft_pc (Utilities|Casting|CastToTestCraft_PC (Game|GetPlayerController 0))
    (:then
      (Variables|Refs|SetTestCraftPC_Ref _astest_craft_pc))
    (:CastFailed
      (bind _asmain_pc (Utilities|Casting|CastToMain_PC (Game|GetPlayerController 0)))
      (Variables|Refs|SetMainPC_Ref _asmain_pc)
      ;[1 1 1] Only for testing
      (bind _asmain_character (Utilities|Casting|CastToMain_Character (Game|GetPlayerCharacter 0)))
      (Variables|Refs|SetChar_Ref _asmain_character))))

(fn TakeinHand
  (Transformation|AttachComponentToComponent (Variables|/Script/Engine.Character|GetMesh (Variables|Refs|GetChar_Ref)) "HoldingSocket" "SnapToTarget" "SnapToTarget" "KeepWorld" true))