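; Base world actor for a grass pickup, showing an action icon while the player character is inside its pickup radius.
; The construction script uses GrassIndex as the DT_AllGrassTypes row name to load attributes and set the pickup mesh.
; Overlaps also bind and unbind the player controller's pickup event, a path marked OLD.
; A legacy function adds the index to the character's inventory and destroys the actor on success.
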(event OnComponentBeginOverlap(PickUpRadius)
  (params (OverlappedComponent :type Primitive%20Component%20Object%20Reference) (OtherActor :type Actor%20Object%20Reference) (OtherComp :type Primitive%20Component%20Object%20Reference) (OtherBodyIndex :type Integer) (bFromSweep :type Boolean) (SweepResult :type Hit%20Result%20Structure%20%28by%20ref%29))
  (Utilities|Casting|CastToBP_Character OtherActor)
  (CallFunction|ShowActionIcon)
  ;[1 1 1] OLD (Bind)
  (EventDispatchers|BindEventtoPickUpD (Variables|Refs|GetPC_Ref) (EventDispatchers|CreateEvent :!event AddtoInventoryOLD)))

(event OnComponentEndOverlap(PickUpRadius)
  (params (OverlappedComponent :type Primitive%20Component%20Object%20Reference) (OtherActor :type Actor%20Object%20Reference) (OtherComp :type Primitive%20Component%20Object%20Reference) (OtherBodyIndex :type Integer))
  (Utilities|Casting|CastToBP_Character OtherActor)
  (CallFunction|HideActionIcon)
  ;[1 1 1] OLD (Bind)
  (EventDispatchers|UnbindallEventsfromPickUpD (Variables|Refs|GetPC_Ref)))

(event EventBeginPlay
  (CallFunction|SetRefs))

(fn ConstructionScript
  (CallFunction|UpdateAttributesfromIndex))

(fn SetRefs
  (bind _asbp_main_pc (Utilities|Casting|CastToBP_MainPC (Game|GetPlayerController 0)))
  (Variables|Refs|SetPC_Ref _asbp_main_pc)
  (bind _asbp_character (Utilities|Casting|CastToBP_Character (Game|GetPlayerCharacter 0)))
  (bind _output_get (Variables|Refs|SetChar_Ref _asbp_character))
  (Variables|Refs|SetInventory_Ref (Variables|/Game/Blueprints/Character/BP_Character.BP_Character_C|GetInventory_Component _output_get)))

(fn UpdateAttributesfromIndex
  (bind _returnvalue (Utilities|GetDataTableRow "/Game/Data/DataTables/DT_AllGrassTypes.DT_AllGrassTypes" (Utilities|String|StringToName (Utilities|String|ToString(Integer) (Variables|Default|GetGrassIndex))))
    (:then
      (bind _output_get (Variables|Default|SetAttributes _returnvalue))
      (Components|StaticMesh|SetStaticMesh (Variables|Default|GetGrassMesh) (.MeshForPickUp (Utilities|Struct|BreakSGrassAttributes _output_get))))))

(fn ShowActionIcon
  (Rendering|SetVisibility (Variables|Default|GetActionIcon) true false))

(fn HideActionIcon
  (Rendering|SetVisibility (Variables|Default|GetActionIcon) false false))

(fn AddtoInventoryOLD
  (bind _success (Default|AddtoInventory (Variables|Refs|GetInventory_Ref) (Variables|Default|GetGrassIndex)))
  (if _success
    (Actor|DestroyActor)))