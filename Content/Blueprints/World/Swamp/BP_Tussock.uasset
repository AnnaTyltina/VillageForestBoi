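; BP_Tussock is a swamp world prop whose mesh moves vertically up and down in a loop after a start delay.
; A timeline drives the mesh's relative Z height, flipping the Up flag on finish to alternate between forward and reverse playback.
; The construction script applies the Mesh variable to the tussock's static mesh component.
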(event Custom|PlayTimeline
  (if (Variables|Default|GetUp)
    (bind _height (Timeline|FloatTimeline PlayFromStart)
      (:Update
        (Transformation|SetRelativeLocation (Variables|Default|GetTussockMesh) (Math|Vector|MakeVector 0.0 0.0 _height) false false))
      (:Finished
        (Variables|Default|SetUp (not (Variables|Default|GetUp)))
        (CallFunction|PlayTimeline)))
    (else
      (Timeline|FloatTimeline ReverseFromEnd))))

(event EventBeginPlay
  (Utilities|FlowControl|Delay (Variables|Default|GetStartDelay))
  (CallFunction|PlayTimeline))

(fn ConstructionScript
  (Components|StaticMesh|SetStaticMesh (Variables|Default|GetTussockMesh) (Variables|Default|GetMesh)))