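; BP_NewZoneTrigger is a world trigger that records when the player enters a new zone.
; On overlap it skips zone index 0, then passes a DoOnce gate before casting the overlapping actor to BP_MainCharacter.
; RememberZone adds the trigger's Index uniquely to NewZonesIndeces on player 0's BP_MainPlayerState.
; Because the gate precedes the cast, any overlapping actor can consume the single firing.
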(event OnComponentBeginOverlap(Trigger)
  (params (OverlappedComponent :type Primitive%20Component%20Object%20Reference) (OtherActor :type Actor%20Object%20Reference) (OtherComp :type Primitive%20Component%20Object%20Reference) (OtherBodyIndex :type Integer) (bFromSweep :type Boolean) (SweepResult :type Hit%20Result%20Structure%20%28by%20ref%29))
  ;[1 1 1] ToAsk: improve (delete)? will check every time...
  (if (not (CallFunction|CheckifZone0))
    (Utilities|FlowControl|DoOnce false
      (:Completed
        ;[1 0 0.6977] Debug
        (Development|PrintString "Enter new zone")
        (Utilities|Casting|CastToBP_MainCharacter OtherActor)
        (CallFunction|RememberZone)))))

(fn ConstructionScript)

(fn CheckifZone0
  (return (== (Variables|Default|GetIndex) 0)))

(fn RememberZone
  (bind _asbp_main_player_state (Utilities|Casting|CastToBP_MainPlayerState (Variables|/Script/Engine.Controller|GetPlayerState (Game|GetPlayerController 0))))
  (Utilities|Array|AddUnique (Variables|/Game/Blueprints/Generic/BP_MainPlayerState.BP_MainPlayerState_C|GetnewZonesIndeces _asbp_main_player_state) (Variables|Default|GetIndex)))