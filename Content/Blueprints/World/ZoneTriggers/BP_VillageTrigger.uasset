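; Village zone trigger that reacts to the main character entering or leaving and swaps which events are bound to the game state's night dispatcher.
; Both overlaps print a debug message, and leaving also unlocks an achievement.
; Two delayed events play HUD subtitles for night inside the village (grandma's call) and night outside it (self call), apparently serving as the swapped night handlers.
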(event OnComponentBeginOverlap(Trigger)
  (params (OverlappedComponent :type Primitive%20Component%20Object%20Reference) (OtherActor :type Actor%20Object%20Reference) (OtherComp :type Primitive%20Component%20Object%20Reference) (OtherBodyIndex :type Integer) (bFromSweep :type Boolean) (SweepResult :type Hit%20Result%20Structure%20%28by%20ref%29))
  (Utilities|Casting|CastToBP_MainCharacter OtherActor)
  ;[1 0 0.7199] Debug
  (Development|PrintString "Добро пожаловать в деревню")
  (EventDispatchers|BindEventtoNightD (.AsBP%20Main%20Game%20State (Utilities|Casting|CastToBP_MainGameState (Game|GetGameState))) (EventDispatchers|CreateEvent :!event Custom|PlayGandmaCall))
  (EventDispatchers|UnbindEventfromNightD (.AsBP%20Main%20Game%20State (Utilities|Casting|CastToBP_MainGameState (Game|GetGameState))) (EventDispatchers|CreateEvent :!event Custom|PlaySelfCall)))

(event OnComponentEndOverlap(Trigger)
  (params (OverlappedComponent :type Primitive%20Component%20Object%20Reference) (OtherActor :type Actor%20Object%20Reference) (OtherComp :type Primitive%20Component%20Object%20Reference) (OtherBodyIndex :type Integer))
  (Utilities|Casting|CastToBP_MainCharacter OtherActor)
  ;[1 0 0.7199] Debug
  (Development|PrintString "Возвращайтесь в деревню ещё")
  (EventDispatchers|UnbindEventfromNightD (.AsBP%20Main%20Game%20State (Utilities|Casting|CastToBP_MainGameState (Game|GetGameState))) (EventDispatchers|CreateEvent :!event Custom|PlayGandmaCall))
  (EventDispatchers|BindEventtoNightD (.AsBP%20Main%20Game%20State (Utilities|Casting|CastToBP_MainGameState (Game|GetGameState))) (EventDispatchers|CreateEvent :!event Custom|PlaySelfCall))
  (Default|UnlockAchievement (Variables|/Game/Blueprints/Generic/BP_MainPC.BP_MainPC_C|GetBP_AchievementsComponent (.AsBP%20Main%20PC (Utilities|Casting|CastToBP_MainPC (Game|GetPlayerController 0)))) "NewEnumerator4"))

(event Custom|PlayGandmaCall
  (Utilities|FlowControl|Delay 3.0)
  (Default|PlaySubtitles (Variables|/Game/Blueprints/Generic/BP_MainPC.BP_MainPC_C|GetHUD_Ref (.AsBP%20Main%20PC (Utilities|Casting|CastToBP_MainPC (Game|GetPlayerController 0)))) "НочьВДеревне"))

(event Custom|PlaySelfCall
  (Utilities|FlowControl|Delay 3.0)
  (Default|PlaySubtitles (Variables|/Game/Blueprints/Generic/BP_MainPC.BP_MainPC_C|GetHUD_Ref (.AsBP%20Main%20PC (Utilities|Casting|CastToBP_MainPC (Game|GetPlayerController 0)))) "НочьВнеДеревни"))

(fn ConstructionScript)