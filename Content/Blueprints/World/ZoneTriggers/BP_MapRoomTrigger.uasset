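; Map room trigger volume that turns widget interaction on for the main character while they are inside it.
; Overlap begin and end on the Trigger component print debug messages, then add or destroy widget interaction on the overlapping BP_MainCharacter.
; Helper functions, unused by these overlap events, fetch the map reference from the first player's BP_MainPlayerState and test whether Index is zero.
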(event OnComponentBeginOverlap(Trigger)
  (params (OverlappedComponent :type Primitive%20Component%20Object%20Reference) (OtherActor :type Actor%20Object%20Reference) (OtherComp :type Primitive%20Component%20Object%20Reference) (OtherBodyIndex :type Integer) (bFromSweep :type Boolean) (SweepResult :type Hit%20Result%20Structure%20%28by%20ref%29))
  ;[1 0 0.6977] Debug
  (Development|PrintString "Enter MAP ROOM")
  (bind _asbp_main_character (Utilities|Casting|CastToBP_MainCharacter OtherActor))
  (Default|AddWidgetInteraction _asbp_main_character))

(event OnComponentEndOverlap(Trigger)
  (params (OverlappedComponent :type Primitive%20Component%20Object%20Reference) (OtherActor :type Actor%20Object%20Reference) (OtherComp :type Primitive%20Component%20Object%20Reference) (OtherBodyIndex :type Integer))
  ;[1 0 0.6977] Debug
  (Development|PrintString "Leave map room")
  (bind _asbp_main_character (Utilities|Casting|CastToBP_MainCharacter OtherActor))
  (Default|DestroyWidgetInteraction _asbp_main_character))

(fn ConstructionScript)

(fn GetMap
  (bind _asbp_main_player_state (Utilities|Casting|CastToBP_MainPlayerState (Variables|/Script/Engine.Pawn|GetPlayerState (Game|GetPlayerCharacter 0))))
  (return (Variables|/Game/Blueprints/Generic/BP_MainPlayerState.BP_MainPlayerState_C|GetMap_Ref _asbp_main_player_state)))

(fn CheckifZone0
  (return (== (Variables|Default|GetIndex) 0)))