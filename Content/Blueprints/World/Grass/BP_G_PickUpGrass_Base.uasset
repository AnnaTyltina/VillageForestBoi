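; Base pickup actor for grass items that the player can add to the inventory.
; Construction sets the mesh from the DT_AllGrass row matching GrassIndex.
; Overlapping PickUpRadius as the main character shows an action icon and binds an event to the player controller's pickup dispatcher, undone on exit.
; TryToAddToInventory passes the grass index to the character's inventory and destroys the actor on success.
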(event OnComponentBeginOverlap(PickUpRadius)
  (params (OverlappedComponent :type Primitive%20Component%20Object%20Reference) (OtherActor :type Actor%20Object%20Reference) (OtherComp :type Primitive%20Component%20Object%20Reference) (OtherBodyIndex :type Integer) (bFromSweep :type Boolean) (SweepResult :type Hit%20Result%20Structure%20%28by%20ref%29))
  (Utilities|Casting|CastToBP_MainCharacter OtherActor)
  (CallFunction|ShowActionIcon)
  ;[1 1 1] Will be different
  (EventDispatchers|BindEventtoPickUpD (.AsBP%20Main%20PC (Utilities|Casting|CastToBP_MainPC (Game|GetPlayerController 0))) (EventDispatchers|CreateEvent :!event TrytoAddtoInventory)))

(event OnComponentEndOverlap(PickUpRadius)
  (params (OverlappedComponent :type Primitive%20Component%20Object%20Reference) (OtherActor :type Actor%20Object%20Reference) (OtherComp :type Primitive%20Component%20Object%20Reference) (OtherBodyIndex :type Integer))
  (Utilities|Casting|CastToBP_MainCharacter OtherActor)
  (CallFunction|HideActionIcon)
  ;[1 1 1] Will be different
  (EventDispatchers|UnbindEventfromPickUpD (.AsBP%20Main%20PC (Utilities|Casting|CastToBP_MainPC (Game|GetPlayerController 0))) (EventDispatchers|CreateEvent :!event TrytoAddtoInventory)))

(event EventBeginPlay
  (CallFunction|SetRefs))

(fn ConstructionScript
  (CallFunction|UpdateAttributesfromIndex))

(fn SetRefs
  (bind _asbp_main_pc (Utilities|Casting|CastToBP_MainPC (Game|GetPlayerController 0)))
  (Variables|Refs|SetPC_Ref _asbp_main_pc)
  (bind _asbp_main_character (Utilities|Casting|CastToBP_MainCharacter (Game|GetPlayerCharacter 0)))
  (bind _output_get (Variables|Refs|SetChar_Ref _asbp_main_character))
  (Variables|Refs|SetInventory_Ref (Variables|/Game/Blueprints/Character/BP_MainCharacter.BP_MainCharacter_C|GetInventory _output_get)))

(fn UpdateAttributesfromIndex
  (bind _returnvalue (Utilities|GetDataTableRow "/Game/Data/DataTables/DT_AllGrass.DT_AllGrass" (Utilities|String|StringToName (Utilities|String|ToString(Integer) (Variables|Default|GetGrassIndex))))
    (:then
      (Components|StaticMesh|SetStaticMesh (Variables|Default|GetGrassMesh) (.MeshForPickUp (Utilities|Struct|BreakSGrassAttributes _returnvalue))))))

(fn ShowActionIcon
  (Development|SetHiddeninGame (Variables|Default|GetActionIcon) false false))

(fn HideActionIcon
  (Development|SetHiddeninGame (Variables|Default|GetActionIcon) true false))

(fn TrytoAddtoInventory
  (bind _success (Default|AddtoInventory (Variables|Refs|GetInventory_Ref) (Variables|Default|GetGrassIndex) 0 "NewEnumerator0"))
  (if _success
    (Actor|DestroyActor)))