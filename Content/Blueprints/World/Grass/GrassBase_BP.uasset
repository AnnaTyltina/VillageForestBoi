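; GrassBase_BP is a clickable grass item that the player can pick up and drop, with test scaffolding still in place.
; Construction picks its static mesh from the Attributes visual form.
; Clicks register it with TestCraft_PC, which gates selection before it attaches to the test character's HoldingSocket.
; Fall runs a timeline that sweeps it toward world Z zero, then detaches it; collision and blanket height remain unhandled.
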(event Custom|Respond
  (Development|PrintString "Was taken")
  (if (Default|CheckifCanbeSelected (Variables|Refs|GetPC_Ref) self)
    (Default|FillSelected (Variables|Refs|GetPC_Ref) self)
    ;[1 1 1] TODO: Move
    (CallFunction|TakeinHand)))

(event Custom|StopResponding
  (Development|PrintString "Was dropped")
  (Transformation|DetachFromComponent (Variables|Default|GetScene) "KeepWorld" "KeepWorld" "KeepWorld" true))

(event Custom|Fall
  (bind _returnvalue (Transformation|GetActorLocation))
  ;[1 1 1] TODO: mind collision or (worse) get CraftBlanket height
  (bind _alpha (Timeline|FallTimeline PlayFromStart)
    (:Update
      (Transformation|SetActorLocation (Math|Vector|MakeVector (.x _returnvalue) (.y _returnvalue) (Math|Float|Lerp (.z _returnvalue) 0.0 _alpha)) true false))
    (:Finished
      (CallFunction|StopResponding))))

(event MouseInput|EventActorOnClicked
  (params (ButtonPressed :type Key%20Structure :default "None"))
  (CallFunction|Respond)
  (Default|FillSelected (Variables|Refs|GetPC_Ref) self))

(event EventBeginPlay
  (CallFunction|SetRefs))

(fn ConstructionScript
  (Components|StaticMesh|SetStaticMesh (Variables|Default|GetStaticMesh) (Utilities|Select :Index (.visualform (Variables|Default|GetAttributes)) :NewEnumerator0 "/Game/Assets/Meshes/1M_Cube.1M_Cube" :NewEnumerator1 "/Game/Testing/TestGrass_Mesh.TestGrass_Mesh" :NewEnumerator2 "/Engine/BasicShapes/Cone.Cone")))

(fn SetRefs
  (bind _astest_craft_pc (Utilities|Casting|CastToTestCraft_PC (Game|GetPlayerController 0)))
  (Variables|Refs|SetPC_Ref _astest_craft_pc)
  ;[1 1 1] Only for testing
  (bind _astest_hand_bp (Utilities|Casting|CastToTestHand_BP (Game|GetPlayerCharacter 0)))
  (Variables|Refs|SetTestHand_Ref _astest_hand_bp))

(fn TakeinHand
  (Transformation|AttachComponentToComponent (Variables|/Script/Engine.Character|GetMesh (Variables|Refs|GetTestHand_Ref)) "HoldingSocket" "SnapToTarget" "SnapToTarget" "KeepWorld" true))