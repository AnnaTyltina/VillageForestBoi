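; BP_Trinket is a world actor with a configurable static mesh, built toward touch-drag rotation but unfinished.
; Helper functions track Touch1 movement, wrap a 2D screen rotation by modulo 360, and convert it into a rotator combined with the actor's rotation.
; None of the drag or rotation logic is wired to events; clicking only prints a debug greeting, and Tick is empty.
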(event EventTick
  (params (DeltaSeconds :type Float%20%28single-precision%29))
  ;[1 1 1] TODO: Handle
)

(event MouseInput|EventActorOnClicked
  (params (ButtonPressed :type Key%20Structure :default "None"))
  (Development|PrintString "Hello"))

(event EventBeginPlay)

(fn ConstructionScript
  (Components|StaticMesh|SetStaticMesh (Variables|Default|GetTrinketMesh) (Variables|Default|GetMesh)))

(fn Rotate
  (bind _returnvalue (Transformation|GetActorRotation))
  (bind _screenrotation (Variables|Default|GetscreenRotation))
  (bind _worldrotation (CallFunction|ConvertScreenRotationtoWorld _screenrotation))
  (bind _returnvalue_2 (Math|Rotator|CombineRotators _worldrotation _returnvalue))
  ;[1 0 0.7553] Debug
  (Development|PrintString (Utilities|String|ToString(Rotator) _returnvalue_2))
  (Transformation|SetActorRotation _returnvalue_2))

(fn StartRotation
  (Variables|Default|SetisRotating true)
  (Variables|Default|SetpreviousPosition (CallFunction|GetClickPosition)))

(fn UpdateDragLength
  (bind _output_get (Variables|Default|SetdragLength (CallFunction|GetDeltaPosition)))
  (Development|PrintString (Utilities|String|ToString(Vector2d) _output_get))
  (Variables|Default|SetpreviousPosition (CallFunction|GetClickPosition)))

(fn ClampScreenRotation
  (params (rotation :type Vector%202D%20Structure))
  (bind (_x _y) (Math|Vector2D|BreakVector2D rotation))
  (return (Math|Vector2D|MakeVector2D (Math|Float|%(Float) _x 3.6e+02) (Math|Float|%(Float) _y 3.6e+02))))

(fn GetClickPosition
  (bind _returnvalue (Game|GetPlayerController 0))
  (bind (_locationx _locationy) (Class|PlayerController|GetInputTouchState _returnvalue "Touch1"))
  (return (Math|Vector2D|MakeVector2D _locationx _locationy)))

(fn GetDeltaPosition
  (return (- (CallFunction|GetClickPosition) (Variables|Default|GetpreviousPosition))))

(fn ConvertScreenRotationtoWorld
  (params (rotation :type Vector%202D%20Structure))
  (LocalVariables|SetAxisZ (.X (Math|Vector2D|BreakVector2D rotation)))
  (LocalVariables|SetAxisXY (CallFunction|YtoXY (.Y (Math|Vector2D|BreakVector2D rotation))))
  (return (Math|Rotator|MakeRotator (.x (LocalVariables|GetAxisXY)) (.y (LocalVariables|GetAxisXY)) (LocalVariables|GetAxisZ))))

(fn YtoXY
  (params (Y :type Float%20%28single-precision%29))
  (return (Class|KismetMathLibrary|GetRotated2D (Math|Vector2D|MakeVector2D 0.0 Y) (- 3.6e+02 Y))))