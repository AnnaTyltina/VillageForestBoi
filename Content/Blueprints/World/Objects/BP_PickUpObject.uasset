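; BP_PickUpObject is a world object that can be picked up into the player's inventory.
; Its ObjectIndex selects a pickup mesh from DT_AllObjects, applied on construction and again after a short BeginPlay delay.
; Radius overlaps with the main character bind and unbind an event on the player controller's pickup dispatcher.
; AddToInventory passes the index to the character's inventory and destroys the actor on success.
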(event OnComponentBeginOverlap(PickUpRadius)
  (params (OverlappedComponent :type Primitive%20Component%20Object%20Reference) (OtherActor :type Actor%20Object%20Reference) (OtherComp :type Primitive%20Component%20Object%20Reference) (OtherBodyIndex :type Integer) (bFromSweep :type Boolean) (SweepResult :type Hit%20Result%20Structure%20%28by%20ref%29))
  (Development|PrintString "PickUpRadius OVERLAP" true true "(R=1.000000,G=0.035601,B=0.000000,A=1.000000)")
  (Utilities|Casting|CastToBP_MainCharacter OtherActor)
  (EventDispatchers|BindEventtoPickUpD (Variables|Refs|GetPC_Ref) (EventDispatchers|CreateEvent :!event AddtoInventory)))

(event OnComponentEndOverlap(PickUpRadius)
  (params (OverlappedComponent :type Primitive%20Component%20Object%20Reference) (OtherActor :type Actor%20Object%20Reference) (OtherComp :type Primitive%20Component%20Object%20Reference) (OtherBodyIndex :type Integer))
  (Development|PrintString "PickUpRadius END overlap" true true "(R=1.000000,G=0.035601,B=0.000000,A=1.000000)")
  (Utilities|Casting|CastToBP_MainCharacter OtherActor)
  (EventDispatchers|UnbindEventfromPickUpD (Variables|Refs|GetPC_Ref) (EventDispatchers|CreateEvent :!event AddtoInventory)))

(event Custom|DestroyPickUpRadius
  (Collision|SetCollisionEnabled (Variables|Default|GetPickUpRadius) "NoCollision"))

(event EventBeginPlay
  (CallFunction|SetRefs)
  ;[1 1 1] TODO: MEHHHHHHH
  (Utilities|FlowControl|Delay 0.1)
  (CallFunction|UpdateAttributes))

(fn ConstructionScript
  (CallFunction|UpdateAttributes))

(fn UpdateAttributes
  (bind _returnvalue (Utilities|GetDataTableRow "/Game/Data/DataTables/DT_AllObjects.DT_AllObjects" (Utilities|String|StringToName (Utilities|String|ToString(Integer) (Variables|Default|GetObjectIndex))))
    (:then
      (Components|StaticMesh|SetStaticMesh (Variables|Default|GetObjectMesh) (.PickUpMesh (Utilities|Struct|BreakSObjectAttributes _returnvalue))))))

(fn SetRefs
  (bind _asbp_main_pc (Utilities|Casting|CastToBP_MainPC (Game|GetPlayerController 0)))
  (Variables|Refs|SetPC_Ref _asbp_main_pc)
  (bind _asbp_main_character (Utilities|Casting|CastToBP_MainCharacter (Game|GetPlayerCharacter 0)))
  (bind _output_get (Variables|Refs|SetChar_Ref _asbp_main_character))
  (Variables|Refs|SetInventory_Ref (Variables|/Game/Blueprints/Character/BP_MainCharacter.BP_MainCharacter_C|GetInventory _output_get)))

(fn AddtoInventory
  (bind _success (Default|AddtoInventory (Variables|Refs|GetInventory_Ref) 0 (Variables|Default|GetObjectIndex) "NewEnumerator1"))
  (if _success
    (Actor|DestroyActor)))

(fn SetInventoryIndex
  (params (InventoryIndex :type Integer))
  (Variables|Default|SetInventoryIndex InventoryIndex))

(fn SetObjectIndex
  (params (ObjectIndex :type Integer))
  (Variables|Default|SetObjectIndex ObjectIndex))