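; Base actor for a craftable grass item that the player clicks to select and hold.
; On BeginPlay it caches player references, binds to the craft-manager-added event and, after a short delay, loads attributes and mesh from a data table by grass index.
; Clicks report the item to the craft manager and, if selectable, attach it to the character's hand socket.
; A timeline-driven Fall lowers it toward zero height, then detaches the mesh.
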(event Custom|Respond
  (Utilities|IsValid (Variables|Refs|GetCraftManager_Ref)
    (:Is%20Valid
      (if (Default|CheckifCanbeSelected (Variables|Refs|GetCraftManager_Ref) self)
        (Default|FillSelected (Variables|/Game/Blueprints/Generic/BP_MainPC.BP_MainPC_C|GetCraftManagerComponent (Variables|Refs|GetMainPC_Ref)) (Utilities|Struct|MakeSClickedGrass (.name (Variables|Default|GetAttributes)) self (Variables|Default|GetInventoryIndex)))
        ;[1 1 1] TODO: Move
        (CallFunction|TakeinHand)))
    (:Is%20Not%20Valid
      (Development|PrintString "Craft Manager is not valid"))))

(event Custom|StopResponding
  (Transformation|DetachFromComponent (Variables|Default|GetGrassMesh) "KeepWorld" "KeepWorld" "KeepWorld" true))

(event Custom|Fall
  (bind _returnvalue (Transformation|GetActorLocation))
  (bind _alpha (Timeline|FallTimeline PlayFromStart)
    (:Update
      (Transformation|SetActorLocation (Math|Vector|MakeVector (.x _returnvalue) (.y _returnvalue) (Math|Float|Lerp (.z _returnvalue) 0.0 _alpha)) true false))
    (:Finished
      (CallFunction|StopResponding))))

(event MouseInput|EventActorOnClicked
  (params (ButtonPressed :type Key%20Structure))
  (CallFunction|Respond)
  (Default|FillSelected (Variables|Refs|GetCraftManager_Ref) (Utilities|Struct|MakeSClickedGrass (.name (Variables|Default|GetAttributes)) self (Variables|Default|GetInventoryIndex))))

(event EventBeginPlay
  (CallFunction|SetRefs)
  (CallFunction|Bind)
  ;[1 1 1] TODO: MEHHHHHHH
  (Utilities|FlowControl|Delay 0.2)
  (CallFunction|UpdateAttributes))

(fn ConstructionScript)

(fn SetRefs
  (bind _asbp_main_pc (Utilities|Casting|CastToBP_MainPC (Game|GetPlayerController 0)))
  (Variables|Refs|SetMainPC_Ref _asbp_main_pc)
  (bind _asbp_character (Utilities|Casting|CastToBP_Character (Game|GetPlayerCharacter 0)))
  (bind _output_get (Variables|Refs|SetChar_Ref _asbp_character))
  (Variables|Refs|SetInventory_Ref (Variables|/Game/Blueprints/Character/BP_Character.BP_Character_C|GetInventory_Component _output_get)))

(fn TakeinHand
  (Transformation|AttachComponentToComponent (Variables|/Script/Engine.Character|GetMesh (Variables|Refs|GetChar_Ref)) "HoldingSocket" "SnapToTarget" "SnapToTarget" "KeepWorld" true))

(fn UpdateCraftManagerRef
  (Variables|Refs|SetCraftManager_Ref (Variables|/Game/Blueprints/Generic/BP_MainPC.BP_MainPC_C|GetCraftManagerComponent (Variables|Refs|GetMainPC_Ref))))

(fn Bind
  (EventDispatchers|BindEventtoOnCraftManagerAddedD (Variables|Refs|GetMainPC_Ref) (EventDispatchers|CreateEvent :!event UpdateCraftManagerRef)))

(fn SetInventoryIndex
  (params (InventoryIndex :type Integer))
  (Variables|Default|SetInventoryIndex InventoryIndex))

(fn UpdateAttributes
  (bind _returnvalue (Utilities|GetDataTableRow "/Game/Data/DataTables/DT_AllGrassTypes.DT_AllGrassTypes" (Utilities|String|StringToName (Utilities|String|ToString(Integer) (Variables|Default|GetGrassIndex))))
    (:then
      (bind _output_get (Variables|Default|SetAttributes _returnvalue))
      (Components|StaticMesh|SetStaticMesh (Variables|Default|GetGrassMesh) (.MeshForCraft (Utilities|Struct|BreakSGrassAttributes _output_get))))))

(fn SetGrassIndex
  (params (GrassIndex :type Integer))
  (Variables|Default|SetGrassIndex GrassIndex))