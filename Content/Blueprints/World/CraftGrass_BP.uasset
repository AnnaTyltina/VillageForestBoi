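; CraftGrass_BP is a world actor for the crafting system that can be selected and dragged through TestCraft_PC.
; Respond prints a click message and passes the actor to the player controller as selected if allowed.
; BeDragged opens a gate on Tick, which snaps the actor to the mouse X/Y at a fixed height, with no close shown.
; The construction script picks the static mesh from Attributes.VisualForm.
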(event Custom|Respond
  (Development|PrintString "Clicked")
  (if (Default|CheckifCanbeSelected (Variables|Default|GetPC_Ref) self)
    (Default|FillSelected (Variables|Default|GetPC_Ref) self)))

(event Custom|BeDragged
  (bind _pc_ref (Variables|Default|GetPC_Ref))
  (bind (_locationx _locationy) (Game|Player|GetMousePosition _pc_ref))
  (Utilities|FlowControl|Gate true) ; enters at Open
)

(event EventTick
  (params (DeltaSeconds :type Float%20%28single-precision%29))
  (bind _pc_ref (Variables|Default|GetPC_Ref))
  (bind (_locationx _locationy) (Game|Player|GetMousePosition _pc_ref))
  (Utilities|FlowControl|Gate true
    (:Exit
      (Transformation|SetActorLocation (Math|Vector|MakeVector _locationx _locationy 1e+02) false false))))

(event EventBeginPlay
  ;[1 1 1] Set Ref
  (bind _astest_craft_pc (Utilities|Casting|CastToTestCraft_PC (Game|GetPlayerController 0)))
  (Variables|Default|SetPC_Ref _astest_craft_pc))

(fn ConstructionScript
  (Components|StaticMesh|SetStaticMesh (Variables|Default|GetStaticMesh) (Utilities|Select :Index (.visualform (Variables|Default|GetAttributes)) :NewEnumerator0 "/Game/Assets/Meshes/1M_Cube.1M_Cube" :NewEnumerator1 "/Game/Assets/Meshes/TestGrass.TestGrass" :NewEnumerator2 "/Engine/BasicShapes/Cone.Cone")))