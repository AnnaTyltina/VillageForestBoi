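; Bowl_BP is a clickable world bowl that receives the item the player last clicked, apparently for crafting.
; On BeginPlay it caches the TestCraft_PC player controller.
; When clicked with a selection, FillBowl stores LastClicked as GrassInBowl and shows its display name on IngredientsText, then the controller's EmptySelectedF is called.
; With no selection it only prints "Nothing to add".
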(event MouseInput|EventActorOnClicked
  (params (ButtonPressed :type Key%20Structure :default "None"))
  (if (== (Variables|/Game/Blueprints/Generic/TestCraft_PC.TestCraft_PC_C|GetlastClicked (Variables|Default|GetPC_Ref)) 0)
    (Development|PrintString "Nothing to add")
    (else
      (CallFunction|FillBowl)
      (Default|EmptySelectedF (Variables|Default|GetPC_Ref)))))

(event EventBeginPlay
  ;[1 1 1] Set Ref
  (bind _astest_craft_pc (Utilities|Casting|CastToTestCraft_PC (Game|GetPlayerController 0)))
  (Variables|Default|SetPC_Ref _astest_craft_pc))

(fn ConstructionScript)

(fn FillBowl
  (bind _output_get (Variables|Default|SetGrassInBowl (Variables|/Game/Blueprints/Generic/TestCraft_PC.TestCraft_PC_C|GetlastClicked (Variables|Default|GetPC_Ref))))
  (Rendering|Components|TextRender|SetText (Variables|Default|GetIngredientsText) (Utilities|Text|ToText(String) (Utilities|GetDisplayName _output_get))))