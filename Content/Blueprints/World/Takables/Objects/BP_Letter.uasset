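; BP_Letter is a world pickup that adds a letter to the main character's inventory.
; Entering its PickUpRadius shows an action icon and binds an event to the player controller's PickUp dispatcher, while leaving hides and unbinds it.
; LetterAction increments the inventory's letters, refreshes the quest inventory widget directly through the controller's HUD reference (flagged for refactor), then destroys the actor.
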(event OnComponentBeginOverlap(PickUpRadius)
  (params (OverlappedComponent :type Primitive%20Component%20Object%20Reference) (OtherActor :type Actor%20Object%20Reference) (OtherComp :type Primitive%20Component%20Object%20Reference) (OtherBodyIndex :type Integer) (bFromSweep :type Boolean) (SweepResult :type Hit%20Result%20Structure%20%28by%20ref%29))
  (Utilities|Casting|CastToBP_MainCharacter OtherActor)
  (CallFunction|ShowActionIcon)
  (EventDispatchers|BindEventtoPickUpD (Variables|Refs|GetPC_Ref) (EventDispatchers|CreateEvent :!event Custom|LetterAction)))

(event OnComponentEndOverlap(PickUpRadius)
  (params (OverlappedComponent :type Primitive%20Component%20Object%20Reference) (OtherActor :type Actor%20Object%20Reference) (OtherComp :type Primitive%20Component%20Object%20Reference) (OtherBodyIndex :type Integer))
  (Utilities|Casting|CastToBP_MainCharacter OtherActor)
  (CallFunction|HideActionIcon)
  (EventDispatchers|UnbindEventfromPickUpD (Variables|Refs|GetPC_Ref) (EventDispatchers|CreateEvent :!event Custom|LetterAction)))

(event Custom|LetterAction
  (Default|AddLetter (Variables|/Game/Blueprints/Character/BP_MainCharacter.BP_MainCharacter_C|GetInventory (Variables|Refs|GetChar_Ref)))
  ;[1 1 1] TODO: refactor
  (Default|UpdateLetters (Variables|/Game/Blueprints/Widgets/WBP_HUD.WBP_HUD_C|GetWBP_QuestInventory (Variables|/Game/Blueprints/Generic/BP_MainPC.BP_MainPC_C|GetHUD_Ref (Variables|Refs|GetPC_Ref))))
  (Actor|DestroyActor))

(event EventBeginPlay
  (CallFunction|SetRefs))

(fn ConstructionScript)

(fn SetRefs
  (bind _asbp_main_pc (Utilities|Casting|CastToBP_MainPC (Game|GetPlayerController 0)))
  (Variables|Refs|SetPC_Ref _asbp_main_pc)
  (bind _asbp_main_character (Utilities|Casting|CastToBP_MainCharacter (Game|GetPlayerCharacter 0)))
  (Variables|Refs|SetChar_Ref _asbp_main_character))

(fn ShowActionIcon
  (Development|SetHiddeninGame (Variables|Default|GetActionIcon) false false))

(fn HideActionIcon
  (Development|SetHiddeninGame (Variables|Default|GetActionIcon) true false))