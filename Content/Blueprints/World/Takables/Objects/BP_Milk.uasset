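; BP_Milk is a world pickup that adds milk to the player character's inventory.
; On BeginPlay it caches the main player controller and character.
; Overlapping its pickup radius toggles an action icon and binds or unbinds an event on the controller's pickup dispatcher.
; MilkAction adds the milk, refreshes the HUD quest inventory widget, then destroys the actor.
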(event OnComponentBeginOverlap(PickUpRadius)
  (params (OverlappedComponent :type Primitive%20Component%20Object%20Reference) (OtherActor :type Actor%20Object%20Reference) (OtherComp :type Primitive%20Component%20Object%20Reference) (OtherBodyIndex :type Integer) (bFromSweep :type Boolean) (SweepResult :type Hit%20Result%20Structure%20%28by%20ref%29))
  (Utilities|Casting|CastToBP_MainCharacter OtherActor)
  (Development|SetHiddeninGame (Variables|Default|GetActionIcon) false false)
  (EventDispatchers|BindEventtoPickUpD (Variables|Default|GetPC_Ref) (EventDispatchers|CreateEvent :!event Custom|MilkAction)))

(event OnComponentEndOverlap(PickUpRadius)
  (params (OverlappedComponent :type Primitive%20Component%20Object%20Reference) (OtherActor :type Actor%20Object%20Reference) (OtherComp :type Primitive%20Component%20Object%20Reference) (OtherBodyIndex :type Integer))
  (Utilities|Casting|CastToBP_MainCharacter OtherActor)
  (Development|SetHiddeninGame (Variables|Default|GetActionIcon) true false)
  (EventDispatchers|UnbindEventfromPickUpD (Variables|Default|GetPC_Ref) (EventDispatchers|CreateEvent :!event Custom|MilkAction)))

(event Custom|MilkAction
  (Default|AddMilk (Variables|/Game/Blueprints/Character/BP_MainCharacter.BP_MainCharacter_C|GetInventory (Variables|Default|GetChar_Ref)))
  (Default|UpdateMilk (Variables|/Game/Blueprints/Widgets/WBP_HUD.WBP_HUD_C|GetWBP_QuestInventory (Variables|/Game/Blueprints/Generic/BP_MainPC.BP_MainPC_C|GetHUD_Ref (Variables|Default|GetPC_Ref))))
  (Actor|DestroyActor))

(event EventBeginPlay
  (CallFunction|SetRefs))

(fn ConstructionScript)

(fn SetRefs
  (bind _asbp_main_pc (Utilities|Casting|CastToBP_MainPC (Game|GetPlayerController 0)))
  (Variables|Default|SetPC_Ref _asbp_main_pc)
  (bind _asbp_main_character (Utilities|Casting|CastToBP_MainCharacter (Game|GetPlayerCharacter 0)))
  (Variables|Default|SetChar_Ref _asbp_main_character))