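; Inventory trinket actor that the player spins by clicking and dragging, with its mesh set directly or looked up by index in DT_AllTrinkets.
; A click stores the mouse position and opens a gate, so Tick applies torque from the drag offset, axes swapped, until ReleaseTrinket closes it.
; Helpers bind that release to BP_MainPC's mouse-released dispatcher.
; A separate touch-based, yaw-only rotation path is unused by the event graph.
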(event Custom|ReleaseTrinket
  (bind _returnvalue (Game|GetPlayerController 0))
  (bind _mouseposition (Variables|Default|GetmousePosition))
  (bind _asbp_main_pc (Utilities|Casting|CastToBP_MainPC _returnvalue))
  (bind (_locationx _locationy) (Game|Player|GetMousePosition _asbp_main_pc))
  (bind _returnvalue_2 (Math|Vector|MakeVector _locationx _locationy 0.0))
  (bind _returnvalue_3 (- _returnvalue_2 _mouseposition))
  (bind (_x _y) (Math|Vector|BreakVector _returnvalue_3))
  (Development|PrintString "Trinket released")
  (Utilities|FlowControl|Gate true) ; enters at Close
)

(event EventTick
  (params (DeltaSeconds :type Float%20%28single-precision%29))
  (bind _returnvalue (Game|GetPlayerController 0))
  (bind _mouseposition (Variables|Default|GetmousePosition))
  (bind _asbp_main_pc (Utilities|Casting|CastToBP_MainPC _returnvalue))
  (bind (_locationx _locationy) (Game|Player|GetMousePosition _asbp_main_pc))
  (bind _returnvalue_2 (Math|Vector|MakeVector _locationx _locationy 0.0))
  (bind _returnvalue_3 (- _returnvalue_2 _mouseposition))
  (bind (_x _y) (Math|Vector|BreakVector _returnvalue_3))
  (Utilities|FlowControl|Gate true
    (:Exit
      (Class|PrimitiveComponent|AddTorqueinDegrees (Variables|Default|GetTrinketMesh) (* (Math|Vector|MakeVector _y 0.0 (* _x -1.0)) 1.0) "None" false))))

(event MouseInput|EventActorOnClicked
  (params (ButtonPressed :type Key%20Structure))
  (bind _returnvalue (Game|GetPlayerController 0))
  (bind _asbp_main_pc (Utilities|Casting|CastToBP_MainPC _returnvalue))
  (bind (_locationx _locationy) (Game|Player|GetMousePosition _asbp_main_pc))
  (bind _returnvalue_2 (Math|Vector|MakeVector _locationx _locationy 0.0))
  (Development|PrintString "Trinket clicked")
  (Variables|Default|SetmousePosition _returnvalue_2)
  (Utilities|FlowControl|Gate true) ; enters at Open
)

(fn ConstructionScript)

(fn BindReleaseTrinket
  (bind _asbp_main_pc (Utilities|Casting|CastToBP_MainPC (Game|GetPlayerController 0)))
  (EventDispatchers|BindEventtoOnMouseReleasedD _asbp_main_pc (EventDispatchers|CreateEvent :!event Custom|ReleaseTrinket)))

(fn SetMesh
  (params (Mesh :type Static%20Mesh%20Object%20Reference))
  (Components|StaticMesh|SetStaticMesh (Variables|Default|GetTrinketMesh) Mesh))

(fn StartRotation
  (Variables|Default|SetisRotating true)
  (Variables|Default|SetpreviousPosition (CallFunction|GetClickPosition)))

(fn Rotate
  ;[1 1 1] ONLY Z ROTATION ENABLED (others didn't work great)
  (Transformation|SetActorRotation (Math|Rotator|CombineRotators (CallFunction|ConvertScreenRotationtoWorld (Variables|Default|GetscreenRotation)) (Transformation|GetActorRotation))))

(fn UnbindReleaseTrinket
  (bind _asbp_main_pc (Utilities|Casting|CastToBP_MainPC (Game|GetPlayerController 0)))
  (EventDispatchers|UnbindEventfromOnMouseReleasedD _asbp_main_pc (EventDispatchers|CreateEvent :!event Custom|ReleaseTrinket)))

(fn UpdateApperancefromIndex
  (params (Index :type Integer))
  (bind _returnvalue (Utilities|GetDataTableRow "/Game/Data/DataTables/DT_AllTrinkets.DT_AllTrinkets" (Utilities|String|StringToName (Utilities|String|ToString(Integer) Index)))
    (:then
      (Components|StaticMesh|SetStaticMesh (Variables|Default|GetTrinketMesh) (.Mesh (Utilities|Struct|BreakSTrinketAttributes _returnvalue))))))

(fn UpdateDragLength
  (Variables|Default|SetdragLength (CallFunction|GetDeltaPosition))
  (Variables|Default|SetpreviousPosition (CallFunction|GetClickPosition)))

(fn ClampScreenRotation
  (params (rotation :type Vector%202D%20Structure))
  (bind (_x _y) (Math|Vector2D|BreakVector2D rotation))
  (return (Math|Vector2D|MakeVector2D (Math|Float|%(Float) _x 3.6e+02) (Math|Float|%(Float) _y 3.6e+02))))

(fn GetClickPosition
  (bind _returnvalue (Game|GetPlayerController 0))
  (bind (_locationx _locationy) (Class|PlayerController|GetInputTouchState _returnvalue "Touch1"))
  (return (Math|Vector2D|MakeVector2D _locationx _locationy)))

(fn GetDeltaPosition
  (return (- (CallFunction|GetClickPosition) (Variables|Default|GetpreviousPosition))))

(fn ConvertScreenRotationtoWorld
  (params (rotation :type Vector%202D%20Structure))
  (LocalVariables|SetAxisZ (.X (Math|Vector2D|BreakVector2D rotation)))
  (LocalVariables|SetAxisXY (CallFunction|YtoXY (.Y (Math|Vector2D|BreakVector2D rotation))))
  (return (Math|Rotator|MakeRotator 0.0 0.0 (LocalVariables|GetAxisZ))))

(fn YtoXY
  (params (Y :type Float%20%28single-precision%29))
  (return (Class|KismetMathLibrary|GetRotated2D (Math|Vector2D|MakeVector2D 0.0 Y) (- 3.6e+02 Y))))