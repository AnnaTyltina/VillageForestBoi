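; BP_PickUpTrinket is a world pickup for a trinket that the player can add to the inventory.
; Its construction script sets the mesh from the DT_AllTrinkets row matching TrinketIndex.
; Overlapping PickUpRadius binds or unbinds a pickup event on the player controller as the main character enters or leaves.
; A successful inventory add shows the new trinket in the HUD backpack menu and destroys the actor.
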(event OnComponentBeginOverlap(PickUpRadius)
  (params (OverlappedComponent :type Primitive%20Component%20Object%20Reference) (OtherActor :type Actor%20Object%20Reference) (OtherComp :type Primitive%20Component%20Object%20Reference) (OtherBodyIndex :type Integer) (bFromSweep :type Boolean) (SweepResult :type Hit%20Result%20Structure%20%28by%20ref%29))
  (Utilities|Casting|CastToBP_MainCharacter OtherActor)
  (EventDispatchers|BindEventtoPickUpD (Variables|Refs|GetPC_Ref) (EventDispatchers|CreateEvent :!event TrytoAddtoInventary)))

(event OnComponentEndOverlap(PickUpRadius)
  (params (OverlappedComponent :type Primitive%20Component%20Object%20Reference) (OtherActor :type Actor%20Object%20Reference) (OtherComp :type Primitive%20Component%20Object%20Reference) (OtherBodyIndex :type Integer))
  (Utilities|Casting|CastToBP_MainCharacter OtherActor)
  (EventDispatchers|UnbindEventfromPickUpD (Variables|Refs|GetPC_Ref) (EventDispatchers|CreateEvent :!event TrytoAddtoInventary)))

(event EventBeginPlay
  (CallFunction|SetRefs))

(fn ConstructionScript
  (CallFunction|UpdateAttributes))

(fn SetRefs
  (Utilities|FlowControl|Sequence
    (:then_0
      (bind _asbp_main_pc (Utilities|Casting|CastToBP_MainPC (Game|GetPlayerController 0)))
      (Variables|Refs|SetPC_Ref _asbp_main_pc))
    (:then_1
      (bind _asbp_main_character (Utilities|Casting|CastToBP_MainCharacter (Game|GetPlayerCharacter 0)))
      (Variables|Refs|SetInventory_Ref (Variables|/Game/Blueprints/Character/BP_MainCharacter.BP_MainCharacter_C|GetInventory _asbp_main_character)))))

(fn UpdateAttributes
  (bind _returnvalue (Utilities|GetDataTableRow "/Game/Data/DataTables/DT_AllTrinkets.DT_AllTrinkets" (Utilities|String|StringToName (Utilities|String|ToString(Integer) (Variables|Default|GetTrinketIndex))))
    (:then
      (Components|StaticMesh|SetStaticMesh (Variables|Default|GetTrinketMesh) (.Mesh (Utilities|Struct|BreakSTrinketAttributes _returnvalue))))))

(fn TrytoAddtoInventary
  (bind _success (Default|AddtoInventory (Variables|Refs|GetInventory_Ref) (Variables|Default|GetTrinketIndex) "NewEnumerator2"))
  (if _success
    (Default|ShowNewTrinket (Variables|/Game/Blueprints/Widgets/Backpack/Trinkets/WBP_Trinkets_Main.WBP_Trinkets_Main_C|GetWBP_TrinketsMenu (Variables|/Game/Blueprints/Widgets/Backpack/WBP_Backpack_Main.WBP_Backpack_Main_C|GetTrinkets (Variables|/Game/Blueprints/Widgets/WBP_HUD.WBP_HUD_C|GetWBP_Backpack_Main (Variables|/Game/Blueprints/Generic/BP_MainPC.BP_MainPC_C|GetHUD_Ref (Variables|Refs|GetPC_Ref))))) (Variables|Default|GetTrinketIndex))
    (Actor|DestroyActor)))