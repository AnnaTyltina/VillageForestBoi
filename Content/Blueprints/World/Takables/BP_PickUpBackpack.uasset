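; BP_PickUpBackpack is a world pickup that gives the player a backpack.
; Overlap with PickUpRadius by BP_MainCharacter shows or hides ActionText and binds or unbinds PickUp on the BP_MainPC pickup dispatcher.
; PickUp sets the backpack flag on the player controller and destroys the actor, with a TODO flagging it for refactoring.
; Disconnected nodes for attaching to the character's Backpack_Socket never run.
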(event OnComponentBeginOverlap(PickUpRadius)
  (params (OverlappedComponent :type Primitive%20Component%20Object%20Reference) (OtherActor :type Actor%20Object%20Reference) (OtherComp :type Primitive%20Component%20Object%20Reference) (OtherBodyIndex :type Integer) (bFromSweep :type Boolean) (SweepResult :type Hit%20Result%20Structure%20%28by%20ref%29))
  (Utilities|Casting|CastToBP_MainCharacter OtherActor)
  (CallFunction|ShowTip)
  (bind _asbp_main_pc (Utilities|Casting|CastToBP_MainPC (Game|GetPlayerController 0)))
  (EventDispatchers|BindEventtoPickUpD _asbp_main_pc (delegate Custom|pickUp)))

(event OnComponentEndOverlap(PickUpRadius)
  (params (OverlappedComponent :type Primitive%20Component%20Object%20Reference) (OtherActor :type Actor%20Object%20Reference) (OtherComp :type Primitive%20Component%20Object%20Reference) (OtherBodyIndex :type Integer))
  (Utilities|Casting|CastToBP_MainCharacter OtherActor)
  (CallFunction|HideTip)
  (bind _asbp_main_pc (Utilities|Casting|CastToBP_MainPC (Game|GetPlayerController 0)))
  (EventDispatchers|UnbindEventfromPickUpD _asbp_main_pc (delegate Custom|pickUp)))

(event Custom|pickUp
  ;[1 1 1] TODO: god why am i so bad at this. i need to _REFACTOR_ this. make. it. better, goddamit
  (bind _asbp_main_pc (Utilities|Casting|CastToBP_MainPC (Game|GetPlayerController 0)))
  (Default|SetHasBackpackTrueREFACTOR _asbp_main_pc)
  (Actor|DestroyActor))

(fn ConstructionScript)

(fn ShowTip
  (Development|SetHiddeninGame (Variables|Default|GetActionText) false false))

(fn HideTip
  (Development|SetHiddeninGame (Variables|Default|GetActionText) true false))