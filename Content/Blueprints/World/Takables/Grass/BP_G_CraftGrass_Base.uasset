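; Base craft grass actor: a clickable grass item that the player can select for crafting and take in hand.
; Its grass index looks up a DT_AllGrass row that supplies the name and inventory mesh, applied at construction and BeginPlay.
; Clicking reports the item to the craft manager and, if selectable, hands it to the character.
; A Fall event detaches the mesh, then sweeps the actor a short distance down via timeline.
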(event OnComponentBeginOverlap(GrassMesh)
  (params (OverlappedComponent :type Primitive%20Component%20Object%20Reference) (OtherActor :type Actor%20Object%20Reference) (OtherComp :type Primitive%20Component%20Object%20Reference) (OtherBodyIndex :type Integer) (bFromSweep :type Boolean) (SweepResult :type Hit%20Result%20Structure%20%28by%20ref%29))
  ;[1 0 0.5689] Debug
  (Development|PrintString "Debug" true true "(R=1.000000,G=0.000000,B=0.360632,A=1.000000)"))

(event Custom|Respond
  (if (Default|CheckifCanbeSelected (Variables|Refs|GetCraftManager_Ref) self)
    (Default|FillSelected (Variables|/Game/Blueprints/Generic/BP_MainPC.BP_MainPC_C|GetCraftManagerComponent (Variables|Refs|GetMainPC_Ref)) (Utilities|Struct|MakeSClickedGrass (.name (Variables|Default|GetAttributes)) self (Variables|Default|GetInventoryIndex)))
    (Default|TakeinHand (Variables|Refs|GetChar_Ref) self)))

(event Custom|StopResponding
  (Transformation|DetachFromComponent (Variables|Default|GetGrassMesh) "KeepWorld" "KeepWorld" "KeepWorld" true))

(event Custom|Fall
  (CallFunction|StopResponding)
  (Variables|Falling|SetFallingStartLocation (Transformation|GetActorLocation))
  (bind _alpha (Timeline|FallTimeline PlayFromStart)
    (:Update
      (Transformation|SetActorLocation (Math|Vector|MakeVector (.X (Math|Vector|BreakVector (Variables|Falling|GetFallingStartLocation))) (.Y (Math|Vector|BreakVector (Variables|Falling|GetFallingStartLocation))) (Math|Float|Lerp (.Z (Math|Vector|BreakVector (Variables|Falling|GetFallingStartLocation))) (- (.Z (Math|Vector|BreakVector (Variables|Falling|GetFallingStartLocation))) 14.0) _alpha)) true false))))

(event MouseInput|EventActorOnClicked
  (params (ButtonPressed :type Key%20Structure))
  (Development|PrintString "Clicked")
  (CallFunction|Respond)
  (Default|FillSelected (Variables|Refs|GetCraftManager_Ref) (Utilities|Struct|MakeSClickedGrass (.name (Variables|Default|GetAttributes)) self (Variables|Default|GetInventoryIndex))))

(event EventBeginPlay
  (CallFunction|SetRefs)
  (CallFunction|UpdateAttributes))

(fn ConstructionScript
  (CallFunction|UpdateAttributes))

(fn SetRefs
  (Utilities|FlowControl|Sequence
    (:then_0
      (bind _asbp_main_pc (Utilities|Casting|CastToBP_MainPC (Game|GetPlayerController 0)))
      (Variables|Refs|SetMainPC_Ref _asbp_main_pc))
    (:then_1
      (bind _asbp_main_character (Utilities|Casting|CastToBP_MainCharacter (Game|GetPlayerCharacter 0)))
      ;[1 1 1] Set Inventory_Ref
      (bind _output_get (Variables|Refs|SetChar_Ref _asbp_main_character))
      (Variables|Refs|SetInventory_Ref (Variables|/Game/Blueprints/Character/BP_MainCharacter.BP_MainCharacter_C|GetInventory _output_get))
      ;[1 1 1] Set CraftManager_Ref
      (Variables|Refs|SetCraftManager_Ref (Variables|/Game/Blueprints/Character/BP_MainCharacter.BP_MainCharacter_C|GetCraftManager (Variables|Refs|GetChar_Ref))))))

(fn SetInventoryIndex
  (params (InventoryIndex :type Integer))
  (Variables|Default|SetInventoryIndex InventoryIndex))

(fn SetGrassIndexandUpdate
  (params (GrassIndex :type Integer))
  (Variables|Default|SetGrassIndex GrassIndex)
  (CallFunction|UpdateAttributes))

(fn UpdateAttributes
  (bind _returnvalue (Utilities|GetDataTableRow "/Game/Data/DataTables/Takables/DT_AllGrass.DT_AllGrass" (Utilities|String|StringToName (Utilities|String|ToString(Integer) (Variables|Default|GetGrassIndex))))
    (:then
      (bind _output_get (Variables|Default|SetAttributes _returnvalue))
      (Components|StaticMesh|SetStaticMesh (Variables|Default|GetGrassMesh) (.MeshInInventory (Utilities|Struct|BreakSGrassAttributes _output_get))))))