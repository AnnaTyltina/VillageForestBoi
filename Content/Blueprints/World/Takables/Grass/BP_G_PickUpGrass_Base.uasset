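; Base actor for pickable grass that grows through stages and can be collected into the player's inventory.
; Grass index selects stages from DT_GrassGrowingStages; the construction script sets the current mesh.
; A looping timer, timed by the starting stage, increments the stage and mesh without a bounds check.
; Player overlap toggles an icon and pickup binding; a successful inventory add destroys the actor and plays a sound.
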(event OnComponentBeginOverlap(PickUpRadius)
  (params (OverlappedComponent :type Primitive%20Component%20Object%20Reference) (OtherActor :type Actor%20Object%20Reference) (OtherComp :type Primitive%20Component%20Object%20Reference) (OtherBodyIndex :type Integer) (bFromSweep :type Boolean) (SweepResult :type Hit%20Result%20Structure%20%28by%20ref%29))
  ;[1 1 1] TODO: make takable_class?? or not (different tryToAdd's)
  (Utilities|Casting|CastToBP_MainCharacter OtherActor)
  (CallFunction|ShowActionIcon)
  (EventDispatchers|BindEventtoPickUpD (Variables|Refs|GetPC_Ref) (EventDispatchers|CreateEvent :!event TrytoAddtoInventory)))

(event OnComponentEndOverlap(PickUpRadius)
  (params (OverlappedComponent :type Primitive%20Component%20Object%20Reference) (OtherActor :type Actor%20Object%20Reference) (OtherComp :type Primitive%20Component%20Object%20Reference) (OtherBodyIndex :type Integer))
  ;[1 1 1] TODO: make takable_class?? or not (different tryToAdd's)
  (Utilities|Casting|CastToBP_MainCharacter OtherActor)
  (CallFunction|HideActionIcon)
  (EventDispatchers|UnbindEventfromPickUpD (Variables|Refs|GetPC_Ref) (EventDispatchers|CreateEvent :!event TrytoAddtoInventory)))

(event Custom|GrowSequence
  ;[1 1 1] Growth Sequence
  (CallFunction|Grow))

(event EventBeginPlay
  (CallFunction|SetRefs)
  ;[1 1 1] Growth Sequence
  (Utilities|Time|SetTimerbyEvent (delegate Custom|GrowSequence) (.Time (CallFunction|GetCurrentStageAttributes)) true))

(fn ConstructionScript
  (CallFunction|UpdateMesh))

(fn SetRefs
  (bind _asbp_main_pc (Utilities|Casting|CastToBP_MainPC (Game|GetPlayerController 0)))
  (Variables|Refs|SetPC_Ref _asbp_main_pc)
  (bind _asbp_main_character (Utilities|Casting|CastToBP_MainCharacter (Game|GetPlayerCharacter 0)))
  (bind _output_get (Variables|Refs|SetChar_Ref _asbp_main_character))
  (Variables|Refs|SetInventory_Ref (Variables|/Game/Blueprints/Character/BP_MainCharacter.BP_MainCharacter_C|GetInventory _output_get)))

(fn UpdateMesh
  (bind _returnvalue (Utilities|GetDataTableRow "/Game/Data/DataTables/DT_GrassGrowingStages.DT_GrassGrowingStages" (Utilities|String|StringToName (Utilities|String|ToString(Integer) (Variables|Default|GetGrassIndex))))
    (:then
      (Components|StaticMesh|SetStaticMesh (Variables|Default|GetGrassMesh) (.Mesh (Utilities|Struct|BreakSGrassGrowingAttributes (Utilities|Array|Get(acopy) (.GrowingStages (Utilities|Struct|BreakSGrassGrowingStages _returnvalue)) (Variables|Default|GetCurrentStage))))))))

(fn ShowActionIcon
  (Development|SetHiddeninGame (Variables|Default|GetActionIcon) false false))

(fn HideActionIcon
  (Development|SetHiddeninGame (Variables|Default|GetActionIcon) true false))

(fn TrytoAddtoInventory
  (bind _success (Default|AddtoInventory (Variables|Refs|GetInventory_Ref) (Variables|Default|GetGrassIndex) "NewEnumerator0"))
  (if _success
    (Actor|DestroyActor)
    (Audio|PlaySound2D "/Game/Assets/Sounds/S_PickGrass.S_PickGrass" 1.0 1.0 0.0 0 0)))

(fn Grow
  (Math|Integer|IncrementInt (Variables|Default|GetCurrentStage)
    (:%20%20
      (CallFunction|UpdateMesh))))

(fn GetGrassStages
  (bind _returnvalue (Utilities|GetDataTableRow "/Game/Data/DataTables/DT_GrassGrowingStages.DT_GrassGrowingStages" (Utilities|String|StringToName (Utilities|String|ToString(Integer) (Variables|Default|GetGrassIndex))))
    (:then
      (return (.GrowingStages (Utilities|Struct|BreakSGrassGrowingStages _returnvalue))))))

(fn GetCurrentStageAttributes
  (bind _growingstages (CallFunction|GetGrassStages))
  (bind _currentstage (Variables|Default|GetCurrentStage))
  (bind _output (Utilities|Array|Get(acopy) _growingstages _currentstage))
  (bind (_stagename _mesh _time) (Utilities|Struct|BreakSGrassGrowingAttributes _output))
  (return _stagename _mesh _time))