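; Village door actor that snaps open or closed according to a per-day opening schedule.
; On BeginPlay it indexes the schedule by the game state's day counter and teleports to a stored open yaw or a closed rotation, flippable via Reversed.
; Doors not flagged OpenForNight also bind to the game state's night and morning dispatchers.
; Helper functions capture the open rotation and load seven schedule entries from DT_Doors, outside the runtime flow.
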(event Custom|Close
  (if (Variables|Default|Getreversed)
    (Transformation|SetActorRotation "0,180.000000, 0" true)
    (else
      (Transformation|SetActorRotation "0, 0, 0" true))))

(event Custom|Open
  (Transformation|SetActorRotation (Math|Rotator|MakeRotator 0.0 0.0 (Variables|Default|GetopenRotation)) true))

(event Custom|switchToDayRotation
  (if (CallFunction|GetIsOpened)
    (CallFunction|Open)
    (else
      (CallFunction|Close))))

(event EventBeginPlay
  (CallFunction|BindEvents)
  (CallFunction|SwitchtoDayRotation))

(fn ConstructionScript)

(fn RememberDayRotation
  (Variables|Default|SetopenRotation (.Yaw (Math|Rotator|BreakRotator (Transformation|GetActorRotation)))))

(fn BindEvents
  (if (not (Variables|Default|GetopenForNight))
    (bind _asbp_main_game_state (Utilities|Casting|CastToBP_MainGameState (Game|GetGameState)))
    (EventDispatchers|BindEventtoNightD _asbp_main_game_state (EventDispatchers|CreateEvent :!event Custom|Close))
    (EventDispatchers|BindEventtoMorningD _asbp_main_game_state (EventDispatchers|CreateEvent :!event Custom|Open))))

(fn RememberOpeningSchedule
  (bind _returnvalue (Utilities|GetDataTableRow "/Game/Data/DataTables/DT_Doors.DT_Doors" (Variables|Default|GetName))
    (:then
      (Variables|Default|SetOpeningSchedule (Utilities|Array|MakeArray (.0 (Utilities|Struct|BreakSDoors _returnvalue)) (.1 (Utilities|Struct|BreakSDoors _returnvalue)) (.2 (Utilities|Struct|BreakSDoors _returnvalue)) (.3 (Utilities|Struct|BreakSDoors _returnvalue)) (.4 (Utilities|Struct|BreakSDoors _returnvalue)) (.5 (Utilities|Struct|BreakSDoors _returnvalue)) (.6 (Utilities|Struct|BreakSDoors _returnvalue)))))))

(fn GetIsOpened
  (return (Utilities|Array|Get(acopy) (Variables|Default|GetOpeningSchedule) (- (Variables|/Game/Blueprints/Generic/BP_MainGameState.BP_MainGameState_C|GetDaysCounter (.AsBP%20Main%20Game%20State (Utilities|Casting|CastToBP_MainGameState (Game|GetGameState)))) 1))))