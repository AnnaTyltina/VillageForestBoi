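; BP_NPC_GuardWoman is an NPC Blueprint for a guard woman who reacts to events from her dialogue.
; Its OnDialogueEvent override matches event names: one sends the player character home through the player controller reference, the other sets a MetGuardWoman flag on the main player state.
; Both cases return false, and BeginPlay and the construction script only call their parents.
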(event EventBeginPlay
  (|CallParentFunction))

(event EventTick
  (params (DeltaSeconds :type Float%20%28single-precision%29))
  (|CallParentFunction DeltaSeconds) ; This node is disabled and will not be called.\nDrag off pins to build functionality.
)

(fn ConstructionScript
  (|CallParentFunction))

(fn OnDialogueEvent
  (params (EventName :type Name%20%28by%20ref%29 :default "None"))
  (switch name EventName
    (:sendHome
      (Default|SendCharHome (Variables|Default|GetPC_Ref))
      (return false))
    (:setMetGuardWoman
      (Variables|/Game/Blueprints/Generic/BP_MainPlayerState.BP_MainPlayerState_C|SetmetGuardWoman (.AsBP%20Main%20Player%20State (Utilities|Casting|CastToBP_MainPlayerState (Variables|/Script/Engine.Pawn|GetPlayerState (Variables|Default|GetChar_Ref)))) true)
      (return false))))