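; Base NPC actor that the player can talk to and receive a quest from.
; Overlapping TalkSpace shows a tip and binds the player controller's talk event, which starts dialogue with this NPC.
; At BeginPlay it selects the first dialogue and, if DT_AllQuests lists its class, caches the row matching QuestIndex.
; Helper functions advance the dialogue and add the quest to the character's QuestManager unless already finished.
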(event OnComponentBeginOverlap(TalkSpace)
  (params (OverlappedComponent :type Primitive%20Component%20Object%20Reference) (OtherActor :type Actor%20Object%20Reference) (OtherComp :type Primitive%20Component%20Object%20Reference) (OtherBodyIndex :type Integer) (bFromSweep :type Boolean) (SweepResult :type Hit%20Result%20Structure%20%28by%20ref%29))
  (Utilities|Casting|CastToBP_MainCharacter OtherActor)
  (CallFunction|ShowTip)
  (EventDispatchers|BindEventtoTalkD (Variables|Refs|GetPC_Ref) (delegate Custom|TalkToNPC)))

(event OnComponentEndOverlap(TalkSpace)
  (params (OverlappedComponent :type Primitive%20Component%20Object%20Reference) (OtherActor :type Actor%20Object%20Reference) (OtherComp :type Primitive%20Component%20Object%20Reference) (OtherBodyIndex :type Integer))
  (Utilities|Casting|CastToBP_MainCharacter OtherActor)
  (CallFunction|HideTip)
  (EventDispatchers|UnbindEventfromTalkD (Variables|Refs|GetPC_Ref) (delegate Custom|TalkToNPC)))

(event Custom|TalkToNPC
  (Default|StartDialogue (Variables|Refs|GetPC_Ref) self))

(event EventBeginPlay
  (CallFunction|SetRefs)
  (CallFunction|UpdateCurrentDialogue)
  ;[1 1 1] Where to put?
  (CallFunction|UpdateQuests))

(fn ConstructionScript)

(fn SetRefs
  (bind _asbp_main_pc (Utilities|Casting|CastToBP_MainPC (Game|GetPlayerController 0)))
  (Variables|Refs|SetPC_Ref _asbp_main_pc)
  (bind _asbp_main_character (Utilities|Casting|CastToBP_MainCharacter (Game|GetPlayerCharacter 0)))
  (bind _output_get (Variables|Refs|SetChar_Ref _asbp_main_character))
  (Variables|Refs|SetQuestManager_Ref (Variables|/Game/Blueprints/Character/BP_MainCharacter.BP_MainCharacter_C|GetQuestManager _output_get)))

(fn ShowTip
  (Development|SetHiddeninGame (Variables|Default|GetTipText) false false))

(fn HideTip
  (Development|SetHiddeninGame (Variables|Default|GetTipText) true false))

(fn AcceptQuest
  (if (CallFunction|CheckifQuestIsComplete)
    (return)
    (else
      (Default|AddQuest (Variables|Refs|GetQuestManager_Ref) (Variables|Default|GetQuestIndex))
      (return))))

(fn UpdateQuests
  (if (CallFunction|CheckifHasAnyQuests)
    (bind _outrownames (DataTable|GetDataTableRowNames "/Game/Data/DataTables/DT_AllQuests.DT_AllQuests"))
    (for _array_element _outrownames
      (bind _returnvalue (Utilities|GetDataTableRow "/Game/Data/DataTables/DT_AllQuests.DT_AllQuests" _array_element)
        (:then
          (LocalVariables|SetRowInCheck_Local _returnvalue)
          (if (== (Variables|Default|GetQuestIndex) (.Index (Utilities|Struct|BreakSAllQuests _returnvalue)))
            (Variables|Default|SetQuestInfo (Utilities|Struct|MakeSQuestInfo (.name (.Quest (Utilities|Struct|BreakSAllQuests (LocalVariables|GetRowInCheck_Local)))) (.type (.Quest (Utilities|Struct|BreakSAllQuests (LocalVariables|GetRowInCheck_Local)))) (.description (.Quest (Utilities|Struct|BreakSAllQuests (LocalVariables|GetRowInCheck_Local)))) (.goal (.Quest (Utilities|Struct|BreakSAllQuests (LocalVariables|GetRowInCheck_Local)))) (.subgoals (.Quest (Utilities|Struct|BreakSAllQuests (LocalVariables|GetRowInCheck_Local))))))
            (return)))))
    (else
      (return))))

(fn UpdateCurrentDialogue
  (Variables|Default|SetCurrentDialogue (Utilities|Array|Get(acopy) (Variables|Default|GetAllDialogues))))

(fn CheckifHasAnyQuests
  (bind _outrownames (DataTable|GetDataTableRowNames "/Game/Data/DataTables/DT_AllQuests.DT_AllQuests"))
  (for _array_element _outrownames
    (bind _returnvalue (Utilities|GetDataTableRow "/Game/Data/DataTables/DT_AllQuests.DT_AllQuests" _array_element)
      (:then
        (if (== (Utilities|GetClass self) (.NPC (Utilities|Struct|BreakSAllQuests _returnvalue)))
          (return true)))))
  (return false))

(fn CheckifQuestIsComplete
  (for _array_element (Variables|/Game/Blueprints/Components/BP_QuestManagerComponent.BP_QuestManagerComponent_C|GetFinishedQuestsIndices (Variables|Refs|GetQuestManager_Ref))
    (if (== _array_element (Variables|Default|GetQuestIndex))
      (return true)))
  (return false))

(fn SwitchtoNextDialogue
  (if (<= (+ (Utilities|Array|FindItem (Variables|Default|GetAllDialogues) (Variables|Default|GetCurrentDialogue)) 1) (Utilities|Array|Length (Variables|Default|GetAllDialogues)))
    (Variables|Default|SetCurrentDialogue (Utilities|Array|Get(acopy) (Variables|Default|GetAllDialogues) (+ (Utilities|Array|FindItem (Variables|Default|GetAllDialogues) (Variables|Default|GetCurrentDialogue)) 1)))
    (else
      (Development|PrintString "Can't switch to next dialogue"))))