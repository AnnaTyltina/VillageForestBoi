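; Farmer NPC Blueprint that supplies the character-specific hooks for the parent NPC's dialogue system.
; OnDialogueEvent handles named events: one shows a new-thing popup and adds the Herbie creature page to the book, another removes the dandelion counter quest tip from the HUD.
; CheckCondition reports whether the farmer quest is closed, read from the character reference.
; Both overrides skip the parent implementations, and the standard event graph is empty.
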(event EventBeginPlay
  (|CallParentFunction) ; This node is disabled and will not be called.\nDrag off pins to build functionality.
)

(event Collision|EventActorBeginOverlap
  (params (OtherActor :type Actor%20Object%20Reference)))

(event EventTick
  (params (DeltaSeconds :type Float%20%28single-precision%29)))

(fn ConstructionScript
  (|CallParentFunction))

(fn OnDialogueEvent
  (params (EventName :type Name%20%28by%20ref%29 :default "None"))
  (switch name EventName
    (:giveHerbiePage
      (Default|ShowNewThing (Variables|/Game/Blueprints/Generic/BP_MainPC.BP_MainPC_C|GetHUD_Ref (Variables|Default|GetPC_Ref)) "NewEnumerator4" 1)
      (Default|AddCreaturePage (Variables|Default|GetBook_Ref) 1)
      (return false))
    (:removeQuestTip
      (Default|DestroyDandelionCounter (Variables|/Game/Blueprints/Generic/BP_MainPC.BP_MainPC_C|GetHUD_Ref (Variables|Default|GetPC_Ref))))))

(fn CheckCondition
  (params (ConditionName :type Name%20%28by%20ref%29 :default "None"))
  (switch name ConditionName
    (:closedFarmerQuest
      (return (Variables|/Game/Blueprints/Character/BP_MainCharacter.BP_MainCharacter_C|GetclosedFarmerQuest (Variables|Default|GetChar_Ref))))))