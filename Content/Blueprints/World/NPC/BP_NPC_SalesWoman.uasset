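; BP_NPC_SalesWoman is a saleswoman NPC that supplies dialogue hooks for quest interactions.
; Its dialogue event handler responds to Give Cookies by adding a cookies quest item to the character's inventory and refreshing the quest inventory HUD widget.
; Its condition check reports whether the milk or cookies quest is active by looking up hardcoded indices in the quest manager's active quest list.
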(event EventBeginPlay
  (|CallParentFunction))

(fn ConstructionScript
  (|CallParentFunction))

(fn OnDialogueEvent
  (params (EventName :type Name%20%28by%20ref%29 :default "None"))
  (switch name EventName
    (:giveCookies
      (Default|AddQuestItem (Variables|/Game/Blueprints/Character/BP_MainCharacter.BP_MainCharacter_C|GetInventory (Variables|Default|GetChar_Ref)) "cookies")
      (Default|UpdateCookies (Variables|/Game/Blueprints/Widgets/WBP_HUD.WBP_HUD_C|GetWBP_QuestInventory (Variables|/Game/Blueprints/Generic/BP_MainPC.BP_MainPC_C|GetHUD_Ref (Variables|Default|GetPC_Ref))))
      (return false))))

(fn CheckCondition
  (params (ConditionName :type Name%20%28by%20ref%29 :default "None"))
  (bind _questmanager_ref (Variables|Default|GetQuestManager_Ref))
  (bind _activequestsindices (Variables|/Game/Blueprints/Components/BP_QuestManagerComponent.BP_QuestManagerComponent_C|GetActiveQuestsIndices _questmanager_ref))
  (switch name ConditionName
    (:hasMilkQuest
      (return (Utilities|Array|ContainsItem _activequestsindices 2)))
    (:hasCookiesQuest
      (return (Utilities|Array|ContainsItem _activequestsindices 5)))))