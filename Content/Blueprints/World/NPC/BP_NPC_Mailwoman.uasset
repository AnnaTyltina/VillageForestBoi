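; BP_NPC_Mailwoman is the mailwoman NPC, supplying the dialogue events and conditions for a letter quest.
; OnDialogueEvent maps named events to flagging the quest as taken on the character, removing all letters from its inventory, or awarding the Mossil creature page to the book with a HUD notification.
; CheckCondition lets dialogue test whether the inventory holds any letters or the full set of at least three.
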(event Custom|TakeLetters
  (Default|RemoveAllLetters (Variables|/Game/Blueprints/Character/BP_MainCharacter.BP_MainCharacter_C|GetInventory (Variables|Default|GetChar_Ref))))

(event EventBeginPlay
  (|CallParentFunction) ; This node is disabled and will not be called.\nDrag off pins to build functionality.
)

(fn ConstructionScript
  (|CallParentFunction))

(fn OnDialogueEvent
  (params (EventName :type Name%20%28by%20ref%29 :default "None"))
  (switch name EventName
    (:tookLettersQuest
      (Variables|/Game/Blueprints/Character/BP_MainCharacter.BP_MainCharacter_C|SettookLettersQuest (Variables|Default|GetChar_Ref) true)
      (return false))
    (:giveMossilPage
      (Default|ShowNewThing (Variables|/Game/Blueprints/Generic/BP_MainPC.BP_MainPC_C|GetHUD_Ref (Variables|Default|GetPC_Ref)) "NewEnumerator4" 2)
      (Default|AddCreaturePage (Variables|Default|GetBook_Ref) 2)
      (return false))
    (:takeLetters
      (CallFunction|TakeLetters)
      (return false))))

(fn CheckCondition
  (params (ConditionName :type Name%20%28by%20ref%29 :default "None"))
  (bind _char_ref (Variables|Default|GetChar_Ref))
  (bind _inventory (Variables|/Game/Blueprints/Character/BP_MainCharacter.BP_MainCharacter_C|GetInventory _char_ref))
  (bind _numberofletters (Default|CountLetters _inventory))
  (switch name ConditionName
    (:hasLetter
      (return (>= _numberofletters 1)))
    (:hasAllLetters
      (return (>= _numberofletters 3)))))