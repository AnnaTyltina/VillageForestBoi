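; BP_NPC_Grandma is the Grandma NPC, who gives the player herb book pages through dialogue.
; The first overlap of the main character with TalkSpace calls TalkToNPC, gated by a DoOnce with no reset.
; OnDialogueEvent maps named dialogue events to custom events that add the Plantain, Nettle or Wind page to BookRef via AddGrassPage, with debug prints.
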(event OnComponentBeginOverlap(TalkSpace)
  (params (OverlappedComponent :type Primitive%20Component%20Object%20Reference) (OtherActor :type Actor%20Object%20Reference) (OtherComp :type Primitive%20Component%20Object%20Reference) (OtherBodyIndex :type Integer) (bFromSweep :type Boolean) (SweepResult :type Hit%20Result%20Structure%20%28by%20ref%29))
  (Utilities|Casting|CastToBP_MainCharacter OtherActor)
  (Utilities|FlowControl|DoOnce false
    (:Completed
      (CallFunction|TalktoNPC))))

(event Custom|GivePlantainPage
  (Default|AddGrassPage (Variables|Default|GetBook_Ref))
  (Development|PrintString "Give PLANTAIN page" true true "(R=1.000000,G=0.384314,B=0.000000,A=1.000000)"))

(event Custom|GiveNettlePage
  (Default|AddGrassPage (Variables|Default|GetBook_Ref) 1)
  (Development|PrintString "Give NETTLE page" true true "(R=1.000000,G=0.384314,B=0.000000,A=1.000000)"))

(event Custom|GiveWindPage
  (Default|AddGrassPage (Variables|Default|GetBook_Ref) 3)
  (Development|PrintString "Give WIND page" true true "(R=1.000000,G=0.384314,B=0.000000,A=1.000000)"))

(event EventBeginPlay
  (|CallParentFunction) ; This node is disabled and will not be called.\nDrag off pins to build functionality.
)

(fn ConstructionScript
  (|CallParentFunction))

(fn OnDialogueEvent
  (params (EventName :type Name%20%28by%20ref%29 :default "None"))
  (switch name EventName
    (:GivePlantainPage
      (CallFunction|GivePlantainPage))
    (:GiveNettlePage
      (CallFunction|GiveNettlePage))
    (:GiveWindPage
      (CallFunction|GiveWindPage)))
  (return false))