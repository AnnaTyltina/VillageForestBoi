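; BP_CraftPlace is a world crafting spot that marks where the main character can craft.
; Its CanCraftTrigger overlap events register the place on BP_MainCharacter when the character enters and clear it when they leave.
; It also exposes functions to toggle or hide a Backpack component and its children in game.
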(event OnComponentBeginOverlap(canCraftTrigger)
  (params (OverlappedComponent :type Primitive%20Component%20Object%20Reference) (OtherActor :type Actor%20Object%20Reference) (OtherComp :type Primitive%20Component%20Object%20Reference) (OtherBodyIndex :type Integer) (bFromSweep :type Boolean) (SweepResult :type Hit%20Result%20Structure%20%28by%20ref%29))
  (bind _asbp_main_character (Utilities|Casting|CastToBP_MainCharacter OtherActor))
  (Default|UpdateCraftPlace _asbp_main_character self))

(event OnComponentEndOverlap(canCraftTrigger)
  (params (OverlappedComponent :type Primitive%20Component%20Object%20Reference) (OtherActor :type Actor%20Object%20Reference) (OtherComp :type Primitive%20Component%20Object%20Reference) (OtherBodyIndex :type Integer))
  (bind _asbp_main_character (Utilities|Casting|CastToBP_MainCharacter OtherActor))
  (Default|ClearCraftPlace _asbp_main_character))

(fn ConstructionScript)

(fn ToggleBackpack
  (bind _backpack (Variables|Default|GetBackpack))
  (Development|SetHiddeninGame _backpack (not (Variables|/Script/Engine.SceneComponent|GetbHiddenInGame _backpack)) true))

(fn HideBackpack
  (Development|SetHiddeninGame (Variables|Default|GetBackpack) true true))