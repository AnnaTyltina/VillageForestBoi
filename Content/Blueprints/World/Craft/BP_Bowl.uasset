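; BP_Bowl is the crafting bowl that collects grass ingredients, counts them on a text display and counts as full at two or more.
; It registers with the player controller and, while the backpack is active, tells the character's CraftManager when craft grass overlaps it.
; FillBowl stores the manager's last-clicked grass.
; Clearing removes those items from the inventory, resets their actors and plays particles, with a delayed variant adding water hiding and a gulp sound.
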(event OnComponentBeginOverlap(BowlSpace)
  (params (OverlappedComponent :type Primitive%20Component%20Object%20Reference) (OtherActor :type Actor%20Object%20Reference) (OtherComp :type Primitive%20Component%20Object%20Reference) (OtherBodyIndex :type Integer) (bFromSweep :type Boolean) (SweepResult :type Hit%20Result%20Structure%20%28by%20ref%29))
  ;[1 1 1] ToAsk: better branch or change collision?
  (if (CallFunction|CheckifCrafting)
    (Utilities|Casting|CastToBP_G_CraftGrass_Base OtherActor)
    (Default|SetIsAboveBowl (Variables|Refs|GetCraftManager_Ref) true)
    (Development|PrintString "isAboveBowl" true true "(R=1.000000,G=0.000000,B=0.337164,A=1.000000)")))

(event OnComponentEndOverlap(BowlSpace)
  (params (OverlappedComponent :type Primitive%20Component%20Object%20Reference) (OtherActor :type Actor%20Object%20Reference) (OtherComp :type Primitive%20Component%20Object%20Reference) (OtherBodyIndex :type Integer))
  ;[1 1 1] ToAsk: better branch or change collision?
  (if (CallFunction|CheckifCrafting)
    (Utilities|Casting|CastToBP_G_CraftGrass_Base OtherActor)
    (Default|SetIsAboveBowl (Variables|Refs|GetCraftManager_Ref) false)
    (Development|PrintString "is_NOT_AboveBowl" true true "(R=1.000000,G=0.000000,B=0.337164,A=1.000000)")))

(event Custom|enableMagicParticle
  ;[1 1 1] Just for fun
  (Components|Activation|Activate (Variables|Default|GetMagicParticle) false))

(event Custom|clearBowlWithEffects
  (Utilities|FlowControl|Delay 1.0)
  (CallFunction|ClearBowl)
  (CallFunction|HideWater)
  (Audio|PlaySound2D "/Game/Assets/Sounds/S_Gulp.S_Gulp" 1.0 1.0 0.0 0 0))

(event EventBeginPlay
  (CallFunction|SetRefs))

(fn ConstructionScript)

(fn SetRefs
  (Utilities|FlowControl|Sequence
    (:then_0
      (bind _asbp_main_pc (Utilities|Casting|CastToBP_MainPC (Game|GetPlayerController 0)))
      (bind _output_get (Variables|Refs|SetMainPC_Ref _asbp_main_pc))
      (Variables|/Game/Blueprints/Generic/BP_MainPC.BP_MainPC_C|SetBowl_Ref _output_get self))
    (:then_1
      (bind _asbp_main_character (Utilities|Casting|CastToBP_MainCharacter (Game|GetPlayerCharacter 0)))
      (bind _output_get_2 (Variables|Refs|SetChar_Ref _asbp_main_character))
      (Variables|Refs|SetInventory_Ref (Variables|/Game/Blueprints/Character/BP_MainCharacter.BP_MainCharacter_C|GetInventory _output_get_2))
      (Variables|Refs|SetCraftManager_Ref (Variables|/Game/Blueprints/Character/BP_MainCharacter.BP_MainCharacter_C|GetCraftManager (Variables|Refs|GetChar_Ref))))))

(fn FillBowl
  (LocalVariables|SetLastClicked_Local (Variables|/Game/Blueprints/Components/BP_CraftManagerComponent.BP_CraftManagerComponent_C|GetLastClicked (Variables|Refs|GetCraftManager_Ref)))
  (Utilities|Array|Add (Variables|Default|GetGrassInBowl) (LocalVariables|GetLastClicked_Local))
  (CallFunction|ShowNumberOfGrass))

(fn ClearBowl
  ;[1 1 1] TODO
  (for _array_element (Variables|Default|GetGrassInBowl)
    (Default|RemoveElement (Variables|Refs|GetInventory_Ref) (.InventoryIndex (Utilities|Struct|BreakSClickedGrass _array_element)))
    (Default|SetGrassIndexandUpdate (.Actor (Utilities|Struct|BreakSClickedGrass _array_element))))
  (CallFunction|EnableMagicParticle)
  (Utilities|Array|Clear (Variables|Default|GetGrassInBowl))
  (CallFunction|ShowNumberOfGrass))

(fn HideWater
  (Rendering|SetVisibility (Variables|Default|GetWater) false false))

(fn ShowGrassNames
  ;[1 0 0.7672] Debug
  (for _array_element (Variables|Default|GetGrassInBowl)
    (Development|PrintString (Utilities|String|Append "IN BOWL: " (Utilities|String|EnumtoString (.Name (Utilities|Struct|BreakSClickedGrass _array_element)))) true true "(R=1.000000,G=0.007519,B=0.000000,A=1.000000)" 5.0)))

(fn ShowNumberOfGrass
  (Rendering|Components|TextRender|SetText (Variables|Default|GetIngredientsText) (Utilities|Text|ToText(String) (Utilities|String|Append (Utilities|String|ToString(Integer) (Utilities|Array|Length (Variables|Default|GetGrassInBowl))) " grass in bowl"))))

(fn ShowWater
  (Rendering|SetVisibility (Variables|Default|GetWater) true false))

(fn CheckifBowlIsFull
  (return (>= (Utilities|Array|Length (Variables|Default|GetGrassInBowl)) 2)))

(fn CheckifCrafting
  ;[1 1 1] ToAsk: is needed?
  (return (Variables|/Game/Blueprints/Character/BP_MainCharacter.BP_MainCharacter_C|GetbackpackIsActive (Variables|Refs|GetChar_Ref))))