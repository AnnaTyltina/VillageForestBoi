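; BP_CraftMenu is an in-world craft menu that displays the player's inventory of grass and objects through Child Actor slots.
; On BeginPlay it caches the player's Inventory and its slot data, registers itself there as CraftMenuRef, then builds its slot arrays.
; For each non-empty inventory slot, it passes item and inventory indices to the matching craft grass or pickup actor.
; Object pickups also lose their pickup radius, a workaround marked TODO.
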(event EventBeginPlay
  (CallFunction|SetRefs)
  (CallFunction|CreateSlotsArray)
  (CallFunction|UpdateInventorySlots))

(fn ConstructionScript)

(fn SetRefs
  ;[1 1 1] Character
  (bind _asbp_main_character (Utilities|Casting|CastToBP_MainCharacter (Game|GetPlayerCharacter 0)))
  (bind _output_get (Variables|Refs|SetChar_Ref _asbp_main_character))
  ;[1 1 1] Inventory
  (Variables|Refs|SetInventory_Ref (Variables|/Game/Blueprints/Character/BP_MainCharacter.BP_MainCharacter_C|GetInventory _output_get))
  ;[1 1 1] Grass In Inventory
  (Variables|Refs|SetGrassInInventory_Ref (Variables|/Game/Blueprints/Components/BP_InventoryComponent.BP_InventoryComponent_C|GetGrassSlots (Variables|Refs|GetInventory_Ref)))
  ;[1 1 1] Objects In Inventory
  (Variables|Refs|SetObjectsInInventory_Ref (Variables|/Game/Blueprints/Components/BP_InventoryComponent.BP_InventoryComponent_C|GetObjectsSlots (Variables|Refs|GetInventory_Ref)))
  ;[1 1 1] CraftMenu
  (Variables|/Game/Blueprints/Components/BP_InventoryComponent.BP_InventoryComponent_C|SetCraftMenu_Ref (Variables|Refs|GetInventory_Ref) self))

(fn UpdateInventorySlots
  (for (_array_element _array_index) (Variables|Default|GetGrassSlots)
    (CallFunction|UpdateGrassSlot _array_index _array_element))
  (for (_array_element_2 _array_index_2) (Variables|Default|GetObjectsSlots)
    (CallFunction|UpdateObjectSlot _array_index_2 _array_element_2)))

(fn UpdateGrassSlot
  (params (Index :type Integer) (Slot :type Child%20Actor%20Component%20Object%20Reference))
  (bind _childactor (Variables|/Script/Engine.ChildActorComponent|GetChildActor Slot))
  (bind _asbp_g_craft_grass_base (Utilities|Casting|CastToBP_G_CraftGrass_Base _childactor))
  (if (Default|IsSlotEmpty (Variables|Refs|GetInventory_Ref) Index "NewEnumerator0")
    (return)
    (else
      (Default|SetGrassIndex _asbp_g_craft_grass_base (.index (Utilities|Array|Get(acopy) (Variables|Refs|GetGrassInInventory_Ref) Index)))
      (Default|SetInventoryIndex _asbp_g_craft_grass_base Index)
      (return))))

(fn UpdateObjectSlot
  (params (Index :type Integer) (Slot :type Child%20Actor%20Component%20Object%20Reference))
  (if (Default|IsSlotEmpty (Variables|Refs|GetInventory_Ref) Index "NewEnumerator1")
    (return)
    (else
      (bind _asbp_pick_up_object (Utilities|Casting|CastToBP_PickUpObject (Variables|/Script/Engine.ChildActorComponent|GetChildActor Slot)))
      (Default|SetObjectIndex _asbp_pick_up_object (.index (Utilities|Array|Get(acopy) (Variables|Refs|GetObjectsInInventory_Ref) Index)))
      (Default|SetInventoryIndex _asbp_pick_up_object Index)
      ;[1 1 1] TODO: solve differently
      (Default|DestroyPickUpRadius _asbp_pick_up_object)
      (return))))

(fn CreateSlotsArray
  (CallFunction|CreateGrassSlotsArray)
  (CallFunction|CreateObjectsSlotsArray))

(fn CreateGrassSlotsArray
  (Variables|Default|SetGrassSlots (Utilities|Array|MakeArray (Variables|Default|GetGrassSlot_1) (Variables|Default|GetGrassSlot_2) (Variables|Default|GetGrassSlot_3) (Variables|Default|GetGrassSlot_4))))

(fn CreateObjectsSlotsArray
  (Variables|Default|SetObjectsSlots (Utilities|Array|MakeArray (Variables|Default|GetOthersSlot_1))))