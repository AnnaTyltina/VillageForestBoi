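; CraftMenu_BP is an early crafting menu Blueprint with child-actor grass slots, tied to the grass items in the player's inventory.
; On BeginPlay, SetRefs casts the player character to Main_Character and stores it along with its InventoryComponent's GrassSlots.
; It then only prints the slot count and each entry's index as debug output, with a rewrite TODO.
; Nodes that would assign the slots' child actor classes are unconnected.
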(event EventBeginPlay
  (CallFunction|SetRefs)
  (Development|PrintString (Utilities|String|ToString(Integer) (Utilities|Array|Length (Variables|Refs|GetGrassInInventory_Ref))) true true "(R=0.000000,G=0.781250,B=0.111734,A=1.000000)")
  ;[1 1 1] TODO: Rewrite
  (for _array_element (Variables|Refs|GetGrassInInventory_Ref)
    (Development|PrintString (Utilities|String|ToString(Name) (.index _array_element)) true true "(R=0.000000,G=0.781250,B=0.111734,A=1.000000)")))

(fn ConstructionScript)

(fn SetRefs
  (bind _asmain_character (Utilities|Casting|CastToMain_Character (Game|GetPlayerCharacter 0)))
  (bind _output_get (Variables|Refs|SetChar_Ref _asmain_character))
  (Variables|Refs|SetGrassInInventory_Ref (Variables|/Game/Blueprints/Components/Inventory_Component.Inventory_Component_C|GetGrassSlots (Variables|/Game/Blueprints/Character/Main_Character.Main_Character_C|GetInventory_Component _output_get))))