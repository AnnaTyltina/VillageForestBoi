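; Bowl_BP is a crafting bowl that collects grass ingredients and registers itself with Main_PC on BeginPlay.
; Filling stores the class of the CraftManagerComponent's last-clicked object, prints the contents' names for debugging and increments a count.
; The bowl reports full at two or more items, can be emptied, and displays a given effect's enum name on its ingredients text.
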(event EventBeginPlay
  (CallFunction|SetRefs))

(fn ConstructionScript)

(fn SetRefs
  (bind _asmain_pc (Utilities|Casting|CastToMain_PC (Game|GetPlayerController 0)))
  (bind _output_get (Variables|Refs|SetMainPC_Ref _asmain_pc))
  (Variables|/Game/Blueprints/Generic/Main_PC.Main_PC_C|SetBowl_Ref _output_get self))

(fn SetCraftManagerRef)

(fn FillBowl
  (Utilities|Array|Add (Variables|Default|GetGrassInBowl) (Utilities|GetClass (Variables|/Game/Blueprints/Components/CraftManager_Component.CraftManager_Component_C|GetLastClicked (Variables|/Game/Blueprints/Generic/Main_PC.Main_PC_C|GetCraftManagerComponent (Variables|Refs|GetMainPC_Ref)))))
  (CallFunction|ShowGrassName)
  (Math|Integer|IncrementInt (Variables|Default|GetAmountOfGrassInBowl)))

(fn EmptyBowl
  (Utilities|Array|Clear (Variables|Default|GetGrassInBowl))
  (Variables|Default|SetAmountOfGrassInBowl 0))

(fn ShowGrassName
  (for _array_element (Variables|Default|GetGrassInBowl)
    (Development|PrintString (Utilities|GetClassDisplayName _array_element) true true "(R=1.000000,G=0.023099,B=0.000000,A=1.000000)")))

(fn ShowGainedEffect
  (params (Effect :type Effects_E%20Enum :default "NewEnumerator0"))
  (Rendering|Components|TextRender|SetText (Variables|Default|GetIngredientsText) (Utilities|Text|ToText(String) (Utilities|String|EnumtoString Effect))))

(fn CheckifBowlIsFull
  (return (>= (Variables|Default|GetAmountOfGrassInBowl) 2)))