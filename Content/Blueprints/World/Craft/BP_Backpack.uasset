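; BP_Backpack is the in-world crafting backpack that displays the player's inventory in physical grass and object slots.
; On BeginPlay it caches the character's inventory, registers itself as its CraftMenuRef and gathers four grass slots and one object slot into arrays.
; Filled inventory entries push their item and slot indices to each slot's child actor.
; It also binds to the player controller's craft-menu-appeared event, marked TODO.
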(event EventBeginPlay
  (CallFunction|SetRefs)
  (CallFunction|CreateSlotsArray)
  (CallFunction|UpdateInventorySlots)
  (bind _asbp_main_pc (Utilities|Casting|CastToBP_MainPC (Game|GetPlayerController 0)))
  ;[1 1 1] TODO
  (EventDispatchers|BindEventtoOnCraftMenuAppearD _asbp_main_pc (EventDispatchers|CreateEvent :!event UpdateInventoryRefs))
  (EventDispatchers|BindEventtoOnCraftMenuAppearD _asbp_main_pc (EventDispatchers|CreateEvent :!event UpdateInventorySlots)))

(fn ConstructionScript)

(fn SetRefs
  ;[1 1 1] Character
  (bind _asbp_main_character (Utilities|Casting|CastToBP_MainCharacter (Game|GetPlayerCharacter 0)))
  (Variables|Refs|SetChar_Ref _asbp_main_character)
  (CallFunction|UpdateInventoryRefs))

(fn UpdateInventoryRefs
  ;[1 1 1] Inventory
  (Variables|Refs|SetInventory_Ref (Variables|/Game/Blueprints/Character/BP_MainCharacter.BP_MainCharacter_C|GetInventory (Variables|Refs|GetChar_Ref)))
  ;[1 1 1] Grass In Inventory
  (Variables|Refs|SetGrassInInventory_Ref (Variables|/Game/Blueprints/Components/BP_InventoryComponent.BP_InventoryComponent_C|GetGrassSlots (Variables|Refs|GetInventory_Ref)))
  ;[1 1 1] Objects In Inventory
  (Variables|Refs|SetObjectsInInventory_Ref (Variables|/Game/Blueprints/Components/BP_InventoryComponent.BP_InventoryComponent_C|GetObjectsSlots (Variables|Refs|GetInventory_Ref)))
  ;[1 1 1] CraftMenu
  (Variables|/Game/Blueprints/Components/BP_InventoryComponent.BP_InventoryComponent_C|SetCraftMenu_Ref (Variables|Refs|GetInventory_Ref) self))

(fn UpdateInventorySlots
  (for (_array_element _array_index) (Variables|Default|GetGrassSlots)
    (CallFunction|UpdateGrassSlot _array_index _array_element))
  (for (_array_element_2 _array_index_2) (Variables|Default|GetObjectsSlots)
    (CallFunction|UpdateObjectSlot _array_index_2 _array_element_2)))

(fn UpdateGrassSlot
  (params (Index :type Integer) (Slot :type Child%20Actor%20Component%20Object%20Reference))
  (bind _grassininventory_ref (Variables|Refs|GetGrassInInventory_Ref))
  (bind _output (Utilities|Array|Get(acopy) _grassininventory_ref Index))
  (bind _childactor (Variables|/Script/Engine.ChildActorComponent|GetChildActor Slot))
  (bind _asbp_g_craft_grass_base (Utilities|Casting|CastToBP_G_CraftGrass_Base _childactor))
  (if (Default|IsSlotEmpty (Variables|Refs|GetInventory_Ref) Index "NewEnumerator0")
    (return)
    (else
      (Default|SetGrassIndexandUpdate _asbp_g_craft_grass_base (.index _output))
      (Default|SetInventoryIndex _asbp_g_craft_grass_base Index)
      ;[1 0 0.6269] Debug
      (Development|PrintString (Utilities|String|Append (Utilities|String|ToString(Integer) Index) " slot filled with " (Utilities|String|EnumtoString (.name _output))) true true "(R=1.000000,G=0.931559,B=0.000000,A=1.000000)")
      (return))))

(fn UpdateObjectSlot
  (params (Index :type Integer) (Slot :type Child%20Actor%20Component%20Object%20Reference))
  (if (Default|IsSlotEmpty (Variables|Refs|GetInventory_Ref) Index "NewEnumerator1")
    (return)
    (else
      (bind _asbp_inventory_object (Utilities|Casting|CastToBP_InventoryObject (Variables|/Script/Engine.ChildActorComponent|GetChildActor Slot)))
      (Default|SetObjectIndexandUpdate _asbp_inventory_object (.index (Utilities|Array|Get(acopy) (Variables|Refs|GetObjectsInInventory_Ref) Index)))
      (Default|SetInventoryIndex _asbp_inventory_object Index)
      (return))))

(fn CreateSlotsArray
  (CallFunction|CreateGrassSlotsArray)
  (CallFunction|CreateObjectsSlotsArray))

(fn CreateGrassSlotsArray
  (Variables|Default|SetGrassSlots (Utilities|Array|MakeArray (Variables|Default|GetGrassSlot_1) (Variables|Default|GetGrassSlot_2) (Variables|Default|GetGrassSlot_3) (Variables|Default|GetGrassSlot_4))))

(fn CreateObjectsSlotsArray
  (Variables|Default|SetObjectsSlots (Utilities|Array|MakeArray (Variables|Default|GetOthersSlot_1))))