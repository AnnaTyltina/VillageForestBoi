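; Test player controller that toggles the ThirdPersonCharacter between a sitting state and its previous state, and triggers crafting while seated.
; The Sit input flip-flops the state and adds a new CraftManager component on every press.
; Releasing left mouse while seated calls Craft on that component.
; Helpers for cursor, camera easing and a duplicate state toggle are uncalled here, and the camera-clamp calls are disconnected.
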(event EventBeginPlay
  (CallFunction|SetRef))

(event Input|ActionEvents|InputActionSit
  (params (Key :type Key%20Structure :default "None"))
  (bind _char_ref (Variables|Default|GetChar_Ref))
  (:Pressed
    (Development|PrintString "Sit")
    (Utilities|FlowControl|FlipFlop
      (:A
        (CallFunction|RememberStateBeforeSitting _char_ref)
        (Default|ChangeState _char_ref "NewEnumerator4"))
      (:B
        (Default|ChangeState (Variables|Default|GetChar_Ref) (Variables|Default|GetstateBeforeSitting))))
    (bind _returnvalue (AddComponent|AddCraftManagerComponent))
    (Variables|Default|SetCraftManagerComponent _returnvalue)))

(event Input|MouseEvents|LeftMouseButton
  (params (Key :type Key%20Structure :default "None"))
  (:Pressed
    ;[1 1 1] TODO: ClampCamera
    (Development|PrintString "ClampCamera" false))
  (:Released
    (if (Utilities|Enum|Equal(Enum) (Variables|/Game/Blueprints/Character/ThirdPersonCharacter.ThirdPersonCharacter_C|GetCurrentState (Variables|Default|GetChar_Ref)) "NewEnumerator4")
      (Default|Craft (Variables|Default|GetCraftManagerComponent)))))

(fn ConstructionScript)

(fn RememberStateBeforeSitting
  (params (character :type Third%20Person%20Character%20Object%20Reference))
  (Variables|Default|SetstateBeforeSitting (Variables|/Game/Blueprints/Character/ThirdPersonCharacter.ThirdPersonCharacter_C|GetCurrentState character)))

(fn SetRef
  (bind _asthird_person_character (Utilities|Casting|CastToThirdPersonCharacter (Game|GetPlayerCharacter 0)))
  (Variables|Default|SetChar_Ref _asthird_person_character))

(fn EnableSittingInterface
  (Variables|Default|SetbShowMouseCursor true)
  ;[1 1 1] TODO: Move
  (CallFunction|SlowCamera))

(fn DisableSittingInterface
  (Input|SetInputModeGameOnly self)
  (Variables|Default|SetbShowMouseCursor false)
  ;[1 1 1] TODO: Move
  (CallFunction|FastenCamera))

(fn SlowCamera
  (Variables|/Game/Blueprints/Character/ThirdPersonCharacter.ThirdPersonCharacter_C|SetCameraUneaseTurn (Variables|Default|GetChar_Ref) 8.0)
  (Variables|/Game/Blueprints/Character/ThirdPersonCharacter.ThirdPersonCharacter_C|SetCameraUneaseLookUp (Variables|Default|GetChar_Ref) 5.0))

(fn FastenCamera
  (Variables|/Game/Blueprints/Character/ThirdPersonCharacter.ThirdPersonCharacter_C|SetCameraUneaseTurn (Variables|Default|GetChar_Ref) 2.0)
  (Variables|/Game/Blueprints/Character/ThirdPersonCharacter.ThirdPersonCharacter_C|SetCameraUneaseLookUp (Variables|Default|GetChar_Ref) 1.0))

(fn SetCameraRotationLimitations
  (params (Camera%20Clamp%20Yaw%20Max :type Float%20%28single-precision%29) (Camera%20Clamp%20Yaw%20Min :type Float%20%28single-precision%29) (Camera%20Clamp%20Pitch%20Max :type Float%20%28single-precision%29) (Camera%20Clamp%20Pitch%20Min :type Float%20%28single-precision%29))
  (Variables|/Game/Blueprints/Character/ThirdPersonCharacter.ThirdPersonCharacter_C|SetCameraClamp (Variables|Default|GetChar_Ref) (Utilities|Struct|MakeCameraClamp_S Camera%20Clamp%20Yaw%20Max Camera%20Clamp%20Yaw%20Min Camera%20Clamp%20Pitch%20Max Camera%20Clamp%20Pitch%20Min)))

(fn HandleStates
  (bind _char_ref (Variables|Default|GetChar_Ref))
  (Utilities|FlowControl|FlipFlop
    (:A
      (Development|PrintString "A" true true "(R=1.000000,G=0.000000,B=0.047059,A=1.000000)")
      (CallFunction|RememberStateBeforeSitting _char_ref)
      (Default|ChangeState _char_ref "NewEnumerator4"))
    (:B
      (Development|PrintString "B" true true "(R=0.635001,G=0.000000,B=1.000000,A=1.000000)")
      (Default|ChangeState (Variables|Default|GetChar_Ref) (Variables|Default|GetstateBeforeSitting)))))