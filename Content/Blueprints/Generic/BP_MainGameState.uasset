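; Game state that runs the repeating Morning, Day, Evening and Night cycle.
; After caching the HUD from the player controller, a delay loop holds each phase for its own length, then advances a wrapping index.
; Each switch plays a HUD transition animation, then fires that phase's dispatcher after a short delay.
; It also binds to the morning dispatcher, and includes a day counter and debug events to set the phase directly.
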(event Custom|switchTimeOfDay
  (bind _index (CallFunction|NextIndex))
  (bind _output_get (Variables|TimeOfDay|SetcurrentTimeOfDay (Utilities|Array|Get(acopy) (Variables|TimeOfDay|GetTimeOfDaySequence) _index)))
  (switch Utilities|FlowControl|Switch|SwitchonETimeOfDay _output_get
    (:NewEnumerator0
      (Default|PlayTimeOfDayAnim (Variables|Refs|GetHUD_Ref) "NewEnumerator0")
      (Utilities|FlowControl|Delay 1.5)
      (Default|CallMorningD))
    (:NewEnumerator1
      (Default|PlayTimeOfDayAnim (Variables|Refs|GetHUD_Ref) "NewEnumerator1")
      (Utilities|FlowControl|Delay 1.5)
      (Default|CallDayD))
    (:NewEnumerator2
      (Default|PlayTimeOfDayAnim (Variables|Refs|GetHUD_Ref) "NewEnumerator2")
      (Utilities|FlowControl|Delay 1.5)
      (Default|CallEveningD))
    (:NewEnumerator3
      (Default|PlayTimeOfDayAnim (Variables|Refs|GetHUD_Ref) "NewEnumerator3")
      (Utilities|FlowControl|Delay 1.5)
      (Default|CallNightD))))

(event Custom|switchToMorning
  ;[1 0 0.7199] Debug only
  (Variables|TimeOfDay|SetcurrentTimeOfDayIndex 0)
  (Variables|TimeOfDay|SetcurrentTimeOfDay "NewEnumerator0"))

(event Custom|incrementDayCounter
  (Math|Integer|IncrementInt (Variables|Default|GetDaysCounter)
    (:%20%20
      ;[1 0 0.7199] Debug
      (Development|PrintString (Utilities|String|Append "CURRENT DAY: " (Utilities|String|ToString(Integer) (Variables|Default|GetDaysCounter))) true true "(R=1.000000,G=0.012991,B=0.000000,A=1.000000)"))))

(event Custom|switchToDay
  ;[1 0 0.7199] Debug only
  (Variables|TimeOfDay|SetcurrentTimeOfDayIndex 1)
  (Variables|TimeOfDay|SetcurrentTimeOfDay "NewEnumerator1"))

(event Custom|switchToEvening
  ;[1 0 0.7199] Debug only
  (Variables|TimeOfDay|SetcurrentTimeOfDayIndex 2)
  (Variables|TimeOfDay|SetcurrentTimeOfDay "NewEnumerator2"))

(event Custom|switchToNight
  ;[1 0 0.7199] Debug only
  (Variables|TimeOfDay|SetcurrentTimeOfDayIndex 3)
  (Variables|TimeOfDay|SetcurrentTimeOfDay "NewEnumerator3"))

(event EventBeginPlay
  (Utilities|FlowControl|Delay 0.2)
  (CallFunction|SetRefs)
  (CallFunction|BindEvents)
  (Utilities|FlowControl|Delay (Variables|TimeOfDay|GetMorningLength))
  ;[1 1 1] TimeOfDay Cycle
  (CallFunction|SwitchTimeOfDay :!label _label)
  (Utilities|FlowControl|Delay (Utilities|Select :Index (Variables|TimeOfDay|GetcurrentTimeOfDay) :NewEnumerator0 (Variables|TimeOfDay|GetMorningLength) :NewEnumerator1 (Variables|TimeOfDay|GetDayLength) :NewEnumerator2 (Variables|TimeOfDay|GetEveningLength) :NewEnumerator3 (Variables|TimeOfDay|GetNightLength)))
  (goto _label))

(fn ConstructionScript)

(fn BindEvents
  (EventDispatchers|BindEventtoMorningD (EventDispatchers|CreateEvent :!event Custom|incrementDayCounter)))

(fn NextIndex
  (bind _output_get (Variables|TimeOfDay|SetcurrentTimeOfDayIndex (Math|Integer|%(Integer) (+ (Variables|TimeOfDay|GetcurrentTimeOfDayIndex) 1) 4)))
  (return _output_get))

(fn SetRefs
  (bind _asbp_main_pc (Utilities|Casting|CastToBP_MainPC (Game|GetPlayerController 0)))
  (Variables|Refs|SetHUD_Ref (Variables|/Game/Blueprints/Generic/BP_MainPC.BP_MainPC_C|GetHUD_Ref _asbp_main_pc)))