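; Prototype player controller for a crafting test where the cursor drives a hand character and clicks grass and a bowl.
; Left press over grass calls its Respond, while release over a bowl calls FillBowl, and every release clears the selection.
; Tick sets the hand anim Blueprint's yaw using look-at from HandSocket to raw screen-pixel mouse coordinates.
; It also debug-prints the cursor's direction relative to the screen-projected shoulder socket.
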(event Custom|FillSelected
  (params (lastClicked :type Craft%20Grass%20BP%20Object%20Reference))
  ;[1 1 1] Not gonna need this
  (bind _output_get (Variables|Default|SetLastClicked lastClicked))
  (Development|PrintString (Utilities|GetDisplayName _output_get)))

(event EventTick
  (params (DeltaSeconds :type Float%20%28single-precision%29))
  (bind (_x_distinction _y_distinction) (CallFunction|MousetoHandCoordinatesDistinction))
  ;[1 1 1] TODO: Refactor
  (CallFunction|SetHandRotation)
  (if (>= _x_distinction 0.0)
    (Development|PrintString "Down")
    (else
      (Development|PrintString "Up")))
  (if (>= _y_distinction 0.0)
    (Development|PrintString "Right")
    (else
      (Development|PrintString "Left"))))

(event EventBeginPlay
  (Input|SetInputModeGameandUI self 0 "DoNotLock" false)
  (CallFunction|SetRefs))

(event Input|MouseEvents|LeftMouseButton
  (params (Key :type Key%20Structure :default "None"))
  (:Pressed
    (bind _ascraft_grass_bp (Utilities|Casting|CastToCraftGrass_BP (.HitActor (Collision|BreakHitResult (.HitResult (Game|Player|GetHitResultUnderCursorbyChannel "TraceTypeQuery1" true))))))
    (Default|Respond _ascraft_grass_bp))
  (:Released
    (Development|PrintString "Released")
    (Utilities|Casting|CastToBowl_BP (.HitActor (Collision|BreakHitResult (.HitResult (Game|Player|GetHitResultUnderCursorbyChannel "TraceTypeQuery1" true))))
      (:then
        (Default|FillBowl (Variables|Default|GetBowl_Ref))
        (CallFunction|EmptySelected))
      (:CastFailed
        (CallFunction|EmptySelected)))))

(fn ConstructionScript)

(fn CheckifSomethingIsSelected
  ;[1 1 1] TODO: Rename
  (if (== (Variables|Default|GetLastClicked) 0)
    (return false)
    (else
      (return true))))

(fn CheckifCanbeSelected
  (params (GrassInCheck :type Craft%20Grass%20BP%20Object%20Reference))
  ;[1 1 1] TODO: Rename
  (LocalVariables|SetGrassInCheck_Local GrassInCheck)
  (if (CallFunction|CheckifSomethingIsSelected)
    (if (== (Variables|Default|GetLastClicked) (LocalVariables|GetGrassInCheck_Local))
      (return true)
      (else
        (return false)))
    (else
      (return true))))

(fn Select
  (params (GrassInCheck :type Craft%20Grass%20BP%20Object%20Reference))
  (if (CallFunction|CheckifCanbeSelected GrassInCheck)
    (CallFunction|EmptySelected)
    (else
      (Development|PrintString "Can't be selected")))
  (return))

(fn EmptySelected
  (Variables|Default|SetLastClicked 0)
  (Development|PrintString "Nothing is selected rn"))

(fn GetSelectedGrass
  (bind _ascraft_grass_bp (Utilities|Casting|CastToCraftGrass_BP (.HitActor (Collision|BreakHitResult (.HitResult (Game|Player|GetHitResultUnderCursorbyChannel "TraceTypeQuery1" true)))))
    (:then
      (return _ascraft_grass_bp))
    (:CastFailed
      (return 0))))

(fn SetRefs
  (bind _astest_craft_pc (Utilities|Casting|CastToTestCraft_PC (Game|GetPlayerController 0)))
  (Variables|Default|SetPC_Ref _astest_craft_pc)
  (bind _astest_hand_bp (Utilities|Casting|CastToTestHand_BP (Game|GetPlayerCharacter 0)))
  (Variables|Default|SetChar_Ref _astest_hand_bp)
  (bind _astest_hand_anim_bp (Utilities|Casting|CastToTestHand_AnimBP (Components|SkeletalMesh|GetAnimInstance (Variables|/Script/Engine.Character|GetMesh (Variables|Default|GetChar_Ref)))))
  (Variables|Default|SetAnimBP_Ref _astest_hand_anim_bp)
  ;[1 1 1] For Testing
  (bind _astest_hand_bp_2 (Utilities|Casting|CastToTestHand_BP (Game|GetPlayerCharacter 0)))
  (Variables|Default|SetTestHand_Ref _astest_hand_bp_2))

(fn SetHandRotation
  (bind (_locationx _locationy) (Game|Player|GetMousePosition))
  (bind _output_get (Variables|/Game/Testing/TestHand_AnimBP.TestHand_AnimBP_C|SetHandRotation (Variables|Default|GetAnimBP_Ref) (Math|Rotator|MakeRotator 0.0 0.0 (* (.yaw (Math|Rotator|FindLookatRotation (Transformation|GetSocketLocation (Variables|/Script/Engine.Character|GetMesh (Variables|Default|GetTestHand_Ref)) "HandSocket") (Math|Vector|MakeVector _locationx _locationy 0.0))) 1.0)))))

(fn MousetoHandCoordinatesDistinction
  (bind _pc_ref (Variables|Default|GetPC_Ref))
  (bind _testhand_ref (Variables|Default|GetTestHand_Ref))
  (bind _pc_ref_2 (Variables|Default|GetPC_Ref))
  (bind (_locationx _locationy) (Game|Player|GetMousePosition _pc_ref_2))
  (bind _mesh (Variables|/Script/Engine.Character|GetMesh _testhand_ref))
  (bind _returnvalue (Transformation|GetSocketLocation _mesh "ShoulderSocket"))
  (bind _screenposition (Class|GameplayStatics|ProjectWorldtoScreen _pc_ref _returnvalue false))
  (return (- _locationy (.y _screenposition)) (- _locationx (.x _screenposition))))