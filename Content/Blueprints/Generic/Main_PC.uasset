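; Player controller for the main character, handling sitting into a crafting mode, pickup input and crafting clicks.
; Sit toggles via FlipFlop: sitting saves state, switches the character, adds a craft manager component and shows the cursor; rising restores state and destroys the component.
; Pickup and manager creation fire dispatchers, while left-click release while crafting calls the manager directly.
; Inventory adding only prints grass table matches; getting up leaves the cursor visible.
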(event EventBeginPlay
  (CallFunction|SetRefs))

(event Input|ActionEvents|InputActionSit
  (params (Key :type Key%20Structure :default "None"))
  (:Pressed
    (Development|PrintString "Sit")
    (Utilities|FlowControl|FlipFlop
      (:A
        ;[1 1 1] TODO: use dispatchers
        (CallFunction|SitDown))
      (:B
        (CallFunction|GetUp)))))

(event Input|ActionEvents|InputActionPickUp
  (params (Key :type Key%20Structure :default "None"))
  (:Pressed
    (Default|CallPickUpD)))

(event Input|MouseEvents|LeftMouseButton
  (params (Key :type Key%20Structure :default "None"))
  (:Released
    ;[1 1 1] TODO: Bind
    (if (Variables|/Game/Blueprints/Character/Main_Character.Main_Character_C|GetisCrafting (Variables|Refs|GetChar_Ref))
      (Default|DecideWhattoDo (Variables|Default|GetCraftManagerComponent)))))

(fn ConstructionScript)

(fn SetRefs
  (bind _asmain_character (Utilities|Casting|CastToMain_Character (Game|GetPlayerCharacter 0)))
  (Variables|Refs|SetChar_Ref _asmain_character))

(fn SetHandRotation)

(fn SetCameraRotationLimitations
  (params (Camera%20Clamp%20Yaw%20Max :type Float%20%28single-precision%29) (Camera%20Clamp%20Yaw%20Min :type Float%20%28single-precision%29) (Camera%20Clamp%20Pitch%20Max :type Float%20%28single-precision%29) (Camera%20Clamp%20Pitch%20Min :type Float%20%28single-precision%29))
  (Variables|/Game/Blueprints/Character/Main_Character.Main_Character_C|SetCameraClamp (Variables|Refs|GetChar_Ref) (Utilities|Struct|MakeCameraClamp_S Camera%20Clamp%20Yaw%20Max Camera%20Clamp%20Yaw%20Min Camera%20Clamp%20Pitch%20Max Camera%20Clamp%20Pitch%20Min)))

(fn AddCraftManager
  (bind _returnvalue (AddComponent|AddCraftManagerComponent))
  (Variables|Default|SetCraftManagerComponent _returnvalue)
  (Default|CallOnCraftManagerAddedD))

(fn AddtoInventory
  (params (RowName :type Name))
  (bind _returnvalue (Utilities|GetDataTableRow "/Game/Data/DataTables/AllGrassTypes_DT.AllGrassTypes_DT" RowName)
    (:then
      (Development|PrintString (Utilities|String|Append "Grass matched: " (Utilities|String|EnumtoString (.name _returnvalue)))))))

(fn HandleStates
  (Utilities|FlowControl|FlipFlop
    (:A
      (Development|PrintString "A" true true "(R=1.000000,G=0.000000,B=0.047059,A=1.000000)")
      (CallFunction|RememberStateBeforeSitting)
      (Default|ChangeState (Variables|Refs|GetChar_Ref) "NewEnumerator4"))
    (:B
      (Development|PrintString "B" true true "(R=0.635001,G=0.000000,B=1.000000,A=1.000000)")
      (Default|ChangeState (Variables|Refs|GetChar_Ref) (Variables|Default|GetstateBeforeSitting)))))

(fn EnableSittingInterface
  (Variables|Default|SetbShowMouseCursor true))

(fn DisableSittingInterface
  (Variables|Default|SetbShowMouseCursor false))

(fn RememberStateBeforeSitting
  (Variables|Default|SetstateBeforeSitting (Variables|/Game/Blueprints/Character/Main_Character.Main_Character_C|GetCurrentState (Variables|Refs|GetChar_Ref))))

(fn DestroyCraftManager
  (Utilities|IsValid (Variables|Default|GetCraftManagerComponent)
    (:Is%20Valid
      (Components|DestroyComponent (Variables|Default|GetCraftManagerComponent)))))

(fn SitDown
  ;[1 1 1] TODO: Refactor
  (CallFunction|RememberStateBeforeSitting)
  (Default|SwitchfromMaintoCraft (Variables|Refs|GetChar_Ref))
  (CallFunction|AddCraftManager)
  (CallFunction|EnableSittingInterface))

(fn GetUp
  ;[1 1 1] TODO: Refactor
  (Default|SwitchfromCrafttoMain (Variables|Refs|GetChar_Ref) (Variables|Default|GetstateBeforeSitting))
  (CallFunction|DestroyCraftManager))