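; Main player controller that owns the HUD and routes input for interaction, backpack, crafting, map updates and NPC dialogue.
; Broadcasts interact and map events through dispatchers, wrapping map updates in a timeline night-widget fade and teleport.
; Backpack toggling seats the character and shows craft or in-game UI by location, while dialogue switches input mode and blends the camera to the NPC.
; Also holds debug keys and unconnected day/night and start-game prototypes.
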(event Custom|FadeIn
  ;[1 1 1] Night/day switching (fade out/in)
  (Widget|SetVisibility (Variables|/Game/Blueprints/Widgets/WBP_HUD.WBP_HUD_C|GetWBP_Night (Variables|Refs|GetHUD_Ref)) "Visible")
  (bind _fadealpha (Timeline|FadeTimeline ReverseFromEnd)
    (:Update
      (Default|UpdateFade (Variables|/Game/Blueprints/Widgets/WBP_HUD.WBP_HUD_C|GetWBP_Night (Variables|Refs|GetHUD_Ref)) _fadealpha))))

(event Custom|FadeOut
  ;[1 1 1] Night/day switching (fade out/in)
  (Widget|SetVisibility (Variables|/Game/Blueprints/Widgets/WBP_HUD.WBP_HUD_C|GetWBP_Night (Variables|Refs|GetHUD_Ref)) "Visible")
  (bind _fadealpha (Timeline|FadeTimeline PlayFromStart)
    (:Update
      (Default|UpdateFade (Variables|/Game/Blueprints/Widgets/WBP_HUD.WBP_HUD_C|GetWBP_Night (Variables|Refs|GetHUD_Ref)) _fadealpha))))

(event EventBeginPlay
  (CallFunction|SetRefs)
  (CallFunction|AddHUD)
  (CallFunction|UnbindAll))

(event Input|ActionEvents|InputActionBackpack
  (params (Key :type Key%20Structure :default "None"))
  (:Pressed
    (if (Variables|Default|GetbackpackIsActive)
      (CallFunction|SwitchtoIngameMode)
      (else
        (CallFunction|SwitchtoBackpackMode)))))

(event Input|ActionEvents|InputActionInteract
  (params (Key :type Key%20Structure :default "None"))
  (:Pressed
    (Default|CallPickUpD)
    (Default|CallTalkD)))

(event Input|ActionEvents|InputActionTryToCraft
  (params (Key :type Key%20Structure :default "None"))
  ;[1 1 1] TODO: rename
  (:Released
    (if (Variables|/Game/Blueprints/Character/BP_MainCharacter.BP_MainCharacter_C|GetbackpackIsActive (Variables|Refs|GetChar_Ref))
      (Default|PerformCraftAction (Variables|Default|GetCraftManagerComponent)))))

(event Input|ActionEvents|InputActionCraft/Book
  (params (Key :type Key%20Structure :default "None"))
  ;[1 0 0.7126] Book Testing
)

(event Input|ActionEvents|InputActionUpdateMap
  (params (Key :type Key%20Structure :default "None"))
  (:Pressed
    ;[1 1 1] ToAsk: MAKE BETTER (bind when enter new zone?)
    (if (Default|CheckifNewZones (Variables|Refs|GetChar_Ref))
      (CallFunction|FadeOut)
      (Utilities|FlowControl|Delay 2.0) ; wait till fade out is finished
      (Default|CallUpdateMapD)
      (Audio|PlaySound2D "/Game/Assets/Music/Environment/Village/S_Env_Bell.S_Env_Bell" 1.0 1.0 0.0 0 0)
      (Default|TeleporttoMap (Variables|Refs|GetChar_Ref))
      (Utilities|FlowControl|Delay 2.0)
      (CallFunction|Fadein)
      (else
        (Development|PrintString "No new zones")))))

(event Input|KeyboardEvents|G
  (params (Key :type Key%20Structure :default "None"))
  ;[1 1 1] FOR NOW
  ; TODO: improve
  (:Pressed
    (Widget|RemovefromParent (Variables|/Game/Blueprints/Widgets/WBP_HUD.WBP_HUD_C|GetWBP_TextCenter (Variables|Refs|GetHUD_Ref)))
    (Default|BlackwithTextFadein (Variables|Refs|GetHUD_Ref))
    (Utilities|FlowControl|Delay 2.0)
    (Default|MovetoGetUpPoint (Variables|Refs|GetChar_Ref))
    (Default|BlackwithTextFadeOut (Variables|Refs|GetHUD_Ref))
    (Utilities|FlowControl|Delay 1.5)
    (Input|SetIgnoreMoveInput false)))

(event Input|KeyboardEvents|LeftShift
  (params (Key :type Key%20Structure :default "None"))
  ;[1 0 0.8589] DEBUG
  (:Pressed
    (Default|SetMaxWalkSpeed (Variables|Refs|GetChar_Ref) 6e+02))
  (:Released
    (Default|SetMaxWalkSpeed (Variables|Refs|GetChar_Ref) 2e+02)))

(event Input|KeyboardEvents|Tab
  (params (Key :type Key%20Structure :default "None"))
  ;[1 0 0.8589] DEBUG
  (:Pressed
    (for _array_element (Variables|/Game/Blueprints/Components/BP_InventoryComponent.BP_InventoryComponent_C|GetObjectsSlots (Variables|/Game/Blueprints/Character/BP_MainCharacter.BP_MainCharacter_C|GetInventory (Variables|Refs|GetChar_Ref)))
      (Development|PrintString (Utilities|String|ToString(Integer) (.Index (Utilities|Struct|BreakSObjectAttributes _array_element)))))))

(event Input|KeyboardEvents|C
  (params (Key :type Key%20Structure :default "None"))
  ;[1 0 0.8589] DEBUG
  (:Pressed
    (Utilities|FlowControl|FlipFlop
      (:A
        (Variables|Default|SetbShowMouseCursor true)
        (Input|SetInputModeGameandUI self 0 "DoNotLock" true))
      (:B
        (Variables|Default|SetbShowMouseCursor false)
        (Input|SetInputModeGameOnly self)))))

(event Input|MouseEvents|LeftMouseButton
  (params (Key :type Key%20Structure :default "None"))
  ;[1 0 0.8589] DEBUG
  (:Pressed
    (Development|PrintString "Pressed")
    (bind _returnvalue (Class|WidgetLayoutLibrary|GetMousePositiononViewport))
    (Variables|Default|SetMouseYValueOnStartDrag (.y _returnvalue)))
  (:Released
    (Development|PrintString "Released")
    (bind _returnvalue_2 (Class|WidgetLayoutLibrary|GetMousePositiononViewport))
    (if (>= (- (Variables|Default|GetMouseYValueOnStartDrag) (.y _returnvalue_2)) 0.2)
      (Development|PrintString (Utilities|String|Append "Drag: " (Utilities|String|ToString(Float) (- (Variables|Default|GetMouseYValueOnStartDrag) (.y _returnvalue_2))))))))

(fn ConstructionScript)

(fn AddHUD
  (UserInterface|Viewport|AddtoViewport (Variables|Refs|GetHUD_Ref) 0))

(fn ChooseCraftorObservation
  (if (CallFunction|CheckifIsinCraftPlace)
    (Default|ShowBackpackCraft (Variables|Refs|GetHUD_Ref))
    (Default|TeleporttoCraftPlace (Variables|Refs|GetChar_Ref))
    (else
      (Default|ShowBackpackIngame (Variables|Refs|GetHUD_Ref)))))

(fn EnableSittingInterface
  (Variables|Default|SetbShowMouseCursor true)
  (Input|SetInputModeGameandUI self 0 "DoNotLock" false))

(fn EndDialogue
  (CallFunction|SetinGameInterface)
  (Default|EnableMovement (Variables|Refs|GetChar_Ref))
  (Game|Player|SetViewTargetwithBlend (Variables|Refs|GetChar_Ref) 0.5 "VTBlend_Linear" 0.0 false)
  ;[1 1 1] TODO: create variable and remember cur NPC
  (bind _outactors (Actor|GetAllActorsOfClass "/Game/Blueprints/World/NPC/BP_MasterNPC.BP_MasterNPC_C"))
  (for _array_element _outactors
    (Default|ShowTip _array_element)))

(fn GetUp
  (Default|SwitchfromCrafttoMain (Variables|Refs|GetChar_Ref) (Variables|Default|GetstateBeforeSitting)))

(fn HideHUD
  ;[1 1 1] TODO: Rename
  (CallFunction|SetinGameInterface))

(fn SetRefs
  (Utilities|FlowControl|Sequence
    (:then_0
      (bind _asbp_main_character (Utilities|Casting|CastToBP_MainCharacter (Game|GetPlayerCharacter 0)))
      (bind _output_get (Variables|Refs|SetChar_Ref _asbp_main_character))
      (Variables|Default|SetCraftManagerComponent (Variables|/Game/Blueprints/Character/BP_MainCharacter.BP_MainCharacter_C|GetCraftManager _output_get)))
    (:then_1
      (bind _returnvalue (UserInterface|CreateWidget "/Game/Blueprints/Widgets/WBP_HUD.WBP_HUD_C"))
      (Variables|Refs|SetHUD_Ref _returnvalue))))

(fn SetinGameInterface
  (Variables|Default|SetbShowMouseCursor false)
  (Input|SetInputModeGameOnly self))

(fn StartDialogue
  (params (NPC :type BP%20Master%20NPC%20Object%20Reference) (DialogueContext :type Dlg%20Context%20Object%20Reference))
  ;[1 1 1] TODO: Rename
  (bind _returnvalue (UserInterface|CreateWidget "/Game/Blueprints/Widgets/Dialogues/WBP_Dialogue_NPC_NewPlugin.WBP_Dialogue_NPC_NewPlugin_C" 0 DialogueContext))
  (UserInterface|Viewport|AddtoViewport _returnvalue 0)
  ;[1 1 1] TODO: extract enable Dialogue/UI Interface function
  (Input|SetInputModeUIOnly self 0 "DoNotLock")
  (Variables|Default|SetbShowMouseCursor true)
  (Pawn|Components|CharacterMovement|DisableMovement (Variables|/Script/Engine.Character|GetCharacterMovement (Variables|Refs|GetChar_Ref)))
  (Default|HideTip NPC)
  (Game|Player|SetViewTargetwithBlend NPC 0.5 "VTBlend_Linear" 0.0 false))

(fn SitDown
  (Default|SwitchfromMaintoCraft (Variables|Refs|GetChar_Ref))
  (Default|CallOnCraftMenuAppearD))

(fn SwitchtoBackpackMode
  (CallFunction|SitDown)
  ;[1 1 1] TODO: rename
  (CallFunction|ChooseCraftorObservation)
  (Variables|Default|SetbackpackIsActive true)
  ;[1 1 1] Not sure
  (Variables|/Game/Blueprints/Character/BP_MainCharacter.BP_MainCharacter_C|SetCurrentMode (Variables|Refs|GetChar_Ref) "NewEnumerator1"))

(fn SwitchtoIngameMode
  (CallFunction|GetUp)
  (Default|HideBackpack (Variables|Refs|GetHUD_Ref))
  (Variables|Default|SetbackpackIsActive false)
  (Variables|/Game/Blueprints/Character/BP_MainCharacter.BP_MainCharacter_C|SetCurrentMode (Variables|Refs|GetChar_Ref) "NewEnumerator0"))

(fn UnbindAll
  ;[1 1 1] ToAsk: if needed
  (EventDispatchers|UnbindallEventsfromPickUpD)
  (EventDispatchers|UnbindallEventsfromTalkD)
  (EventDispatchers|UnbindallEventsfromUpdateMapD)
  (EventDispatchers|UnbindallEventsfromOnCraftMenuAppearD))

(fn CheckifIsinCraftPlace
  (return (Variables|/Game/Blueprints/Character/BP_MainCharacter.BP_MainCharacter_C|GetisInCraftPlace (.AsBP%20Main%20Character (Utilities|Casting|CastToBP_MainCharacter (Game|GetPlayerCharacter 0))))))