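; Text style helper library that converts text with opening-only style tags into fully closed markup, as used by rich text.
; ToTargetText prepends a Normal tag when the text does not start with a tag.
; It then inserts a closing tag before every opening bracket, chops the surplus leading one and appends a final closing tag.
; Each style tag therefore applies until the next one begins.
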(fn ToTargetText
  (params (inText :type Text))
  (LocalVariables|SetprocessedString (Utilities|String|ToString(Text) inText))
  (Utilities|FlowControl|Sequence
    (:then_0
      ;[1 1 1] Make sure text starts with the openning tag
      (if (not (Utilities|String|StartsWith (LocalVariables|GetprocessedString) "<"))
        (LocalVariables|SetprocessedString (Utilities|String|Append "<Normal>" (LocalVariables|GetprocessedString)))))
    (:then_1
      ;[1 1 1] Close middle tags
      (Class|KismetStringLibrary|ReplaceInline (LocalVariables|GetprocessedString) "<" "</><" "IgnoreCase")
      (LocalVariables|SetprocessedString (Utilities|String|RightChop (LocalVariables|GetprocessedString) 3)))
    (:then_2
      ;[1 1 1] Close last tag
      (LocalVariables|SetprocessedString (Utilities|String|Append (LocalVariables|GetprocessedString) "</>")))
    (:then_3
      (return (Utilities|Text|ToText(String) (LocalVariables|GetprocessedString))))))